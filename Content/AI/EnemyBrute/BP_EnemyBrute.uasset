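; BP_EnemyBrute is an AI melee enemy character that takes damage and can be knocked back.
; TakeDamage subtracts from Health and destroys the actor at zero or below.
; Knockback launches it using CalculateKBDir, which scales the unnormalized horizontal offset from the source, so distance increases force, and adds vertical lift.
; AIMeleeAttack and AIAttackTrace are empty; the attack montage and debug capsule trace are disconnected and never run.
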(event `/Game/AI/EnemyFootsoldier/BPI_AICombat.AIMeleeAttack`)

(event `/Game/Assets/BluePrints/Interfaces/BPIDamageRecievers.TakeDamage`
  (params (`Damage Taken` :type "Float (double-precision)"))
  (bind _output_get (set `self.Health` (- (`self.Health`) `Damage Taken`)))
  (if (<= _output_get 0.0)
    (`self.K2_DestroyActor`)))

(event `/Game/Assets/BluePrints/Interfaces/BPIDamageRecievers.Knockback`
  (params (KnockbackSource :type "Vector Structure") (KnockbackValue :type "Float (double-precision)") (`Launch Value` :type "Float (double-precision)"))
  (bind _applied_knockback (`self.Calculate KB Dir` KnockbackSource (`self.K2_GetActorLocation` self) KnockbackValue `Launch Value`))
  (`self.LaunchCharacter` _applied_knockback false true))

(event `AI Attack Trace`
  ;[1 1 1] AI Attack Sphere Trace
)

(fn `Calculate KB Dir`
  (params (`Knockback Source` :type "Vector Structure") (`My Position` :type "Vector Structure") (`Directional Strenght` :type "Float (double-precision)") (`Launch Strenght` :type "Float (double-precision)"))
  (returns (`Applied Knockback` :type "Vector Structure"))
  (locals (NewLocalVar :type "Float (double-precision)") (KnockbackDirection :type "Vector Structure"))
  (bind (_kbs_x _kbs_y _kbs_z) (`KismetMathLibrary.BreakVector` (`self.KBS`)))
  (bind (_mypos_x _mypos_y _mypos_z) (`KismetMathLibrary.BreakVector` (`self.MYPOS`)))
  (set `self.KBS` `Knockback Source`)
  (set `self.MYPOS` `My Position`)
  (bind _output_get (set `local.KnockbackDirection` (+ (`KismetMathLibrary.MakeVector` 0.0 0.0 `Launch Strenght`) (* `Directional Strenght` (- (- (`self.MYPOS`) (`KismetMathLibrary.MakeVector` 0.0 0.0 _mypos_z)) (- (`self.KBS`) (`KismetMathLibrary.MakeVector` 0.0 0.0 _kbs_z)))))))
  (return _output_get))

(fn `UserConstructionScript`)