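; Prototype AI enemy that spots the player character and runs a placeholder forward attack check.
; Pawn sensing sets the "hasSeenPlayer?" blackboard flag on its AI controller when it sees BP_MainCharacter, with no logic here to clear it.
; AttackPlayer sphere-traces ahead against Vehicle objects with persistent debug drawing, printing a message on hitting the player but applying no damage.
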(event `self.PawnSensing.OnSeePawn`
  (params (Pawn :type "Pawn Object Reference"))
  (cast `/Game/Assets/BluePrints/MainCharacter/BP_MainCharacter` Pawn)
  (`BlackboardComponent.SetValueAsBool` (`AIBlueprintHelperLibrary.GetBlackboard` (`AIBlueprintHelperLibrary.GetAIController` self)) "hasSeenPlayer?" true))

(event `Attack Player`
  (bind _returnvalue (`self.K2_GetActorLocation`))
  (bind (_outhit _returnvalue_2) (`KismetSystemLibrary.SphereTraceSingleForObjects` :`Start` _returnvalue :`End` (+ _returnvalue (* (`KismetMathLibrary.GetForwardVector` (`self.K2_GetActorRotation`)) 250.0)) :`Radius` 100.0 :`ObjectTypes` (`|MakeArray` "ObjectTypeQuery5" :!type "EObjectTypeQuery Enum") :`DrawDebugType` "Persistent"))
  (if _returnvalue_2
    (cast `/Game/Assets/BluePrints/MainCharacter/BP_MainCharacter` (`.HitActor` (`GameplayStatics.BreakHitResult` _outhit)))
    (`KismetSystemLibrary.PrintString` "Enemy Attacked Player")))

(fn `UserConstructionScript`)