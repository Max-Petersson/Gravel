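; BP_Turret is a golem turret enemy that rises from the ground, registers with BP_WaveManager and deregisters on death.
; Once risen, it line-traces to the player, turns toward them when visible and runs a delayed, charged attack.
; The attack drops BP_IndicatorForAoe on traced ground at a random point near the player.
; Hits trigger flash, alternating montages, hitstop and camera shake, with hit-counted knockback unless immovable.
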(event `self.ReceiveBeginPlay`
  (bind _asbp_main_character (cast `/Game/Assets/BluePrints/MainCharacter/BP_MainCharacter` (`GameplayStatics.GetPlayerCharacter` 0)))
  (set `self.As BP Main Character` _asbp_main_character)
  (bind _returnvalue (`GameplayStatics.GetActorOfClass` "/Game/AI/WaveLogic/BP_WaveManager.BP_WaveManager_C"))
  (`/Engine/EditorBlueprintResources/StandardMacros.IsValid` _returnvalue
    (:`Is Valid`
      (`/Game/AI/WaveLogic/BP_WaveManager.AddToNeeded` _returnvalue))
    (:`Is Not Valid`
      _))
  (`SceneComponent.K2_SetRelativeLocation` (`self.Mesh`) (0.0 0.0 -500.0) false false)
  (`KismetSystemLibrary.Delay` (`KismetMathLibrary.RandomFloatInRange` 0.5 1.0))
  (`NiagaraFunctionLibrary.SpawnSystemAtLocation` "/Game/Assets/VFX/Enemy_VFX/NS_RisingCloud.NS_RisingCloud" (- (`self.K2_GetActorLocation`) (0.0 0.0 130.0)))
  (bind (_direction _rising_effect) (`Timeline|Rising`)
    (:`Update`
      (`SceneComponent.K2_SetRelativeLocation` (`self.Mesh`) (`KismetMathLibrary.MakeVector` 0.0 0.0 _rising_effect) false false))
    (:`Finished`
      (set `self.Intro` false))))

(event `self.ReceiveTick`
  (params (DeltaSeconds :type "Float (single-precision)"))
  (bind (_returnvalue_roll _returnvalue_pitch _returnvalue_yaw) (`KismetMathLibrary.BreakRotator` (`KismetMathLibrary.RInterpTo` (`self.K2_GetActorRotation`) (`KismetMathLibrary.FindLookAtRotation` (`self.K2_GetActorLocation`) (`self.K2_GetActorLocation` (`self.As BP Main Character`))) (`GameplayStatics.GetWorldDeltaSeconds`))))
  ;[1 1 1] Looks at player
  (if (not (`self.Intro`))
    (bind _outhit (`KismetSystemLibrary.LineTraceSingle` (+ (`self.K2_GetActorLocation`) (0.0 0.0 100.0)) (+ (`self.K2_GetActorLocation` (`self.As BP Main Character`)) (0.0 0.0 50.0)) "TraceTypeQuery1"))
    (bind _output_get (set `self.Sees Player?` (== (`self.As BP Main Character`) (`.HitActor` (`GameplayStatics.BreakHitResult` _outhit)))))
    (if _output_get
      (`self.K2_SetActorRotation` (`KismetMathLibrary.MakeRotator` 0.0 0.0 _returnvalue_yaw))
      (`self.ThrowRock`))))

(event `HitParticleEffects`
  (bind _returnvalue (`SceneComponent.K2_GetComponentLocation` (`self.CapsuleComponent`)))
  ;[1 1 1] Hurt Particles
  (`NiagaraFunctionLibrary.SpawnSystemAtLocation` "/Game/Assets/VFX/Enemy_VFX/NS_ImpactEffect.NS_ImpactEffect" (`KismetMathLibrary.RandomPointInBoundingBox` _returnvalue (50.0 50.0 50.0)))
  (`NiagaraFunctionLibrary.SpawnSystemAtLocation` "/Game/Assets/VFX/Enemy_VFX/NS_MinorStoneBurst.NS_MinorStoneBurst" _returnvalue))

(event `HurtHighlight`
  (bind _mesh (`self.Mesh`))
  ;[1 1 1] Hurt Highlight
  (`PrimitiveComponent.SetMaterial` _mesh 0 "/Game/Assets/Materials/Enemies/M_HurtHighlight.M_HurtHighlight")
  (`KismetSystemLibrary.Delay` 0.2)
  (`PrimitiveComponent.SetMaterial` _mesh 0 "/Game/Assets/Meshes/Enemies/Golem/Golem_material2.Golem_material2"))

(event `ThrowRock`
  ;[0.1498 0.1373 0.5365] Throw Rock
  (`KismetSystemLibrary.Delay` (`KismetMathLibrary.RandomFloatInRange` (`self.MinTimeToThrow`) (`self.MaxTimeToThrow`)))
  (if (`self.Sees Player?`)
    (`ActorComponent.Activate` (`self.NS_EnemyCharging`) false)
    (set `self.NiagraVis` null)
    (set `self.Can Fire?` true)
    (`KismetSystemLibrary.Delay` 1.5) ; This is the stun window
    (if (`self.Can Fire?`)
      (`self.PlayAnimMontage` "/Game/Assets/Animations/Enemies/Ranged/AM_RangedFIre.AM_RangedFIre")
      (`self.SpawnExplosion`))
    (else
      (set `self.Can Fire?` true))))

(event `/Game/Assets/BluePrints/Interfaces/BPIDamageRecievers.TakeDamage`
  (params (`Damage Taken` :type "Float (double-precision)") (PoiseDamage :type "Float (double-precision)"))
  (bind _returnvalue (`self.K2_GetActorLocation` self))
  (bind _returnvalue_2 (`SceneComponent.K2_GetComponentLocation` (`self.CapsuleComponent`)))
  ;[1 1 1] Damage and knockback
  (if (`self.Can Take Damage?`)
    (`self.HurtHighlight`)
    (`/Engine/EditorBlueprintResources/StandardMacros.FlipFlop`
      (:`A`
        (`self.PlayAnimMontage` "/Game/Assets/Animations/Enemies/AM_GolemTakeDamageLeft.AM_GolemTakeDamageLeft"))
      (:`B`
        (`self.PlayAnimMontage` "/Game/Assets/Animations/Enemies/AM_GolemTakeDamageRight.AM_GolemTakeDamageRight")))
    (`GameplayStatics.PlaySoundAtLocation` "/Game/SoundFX/EnemyHit.EnemyHit" _returnvalue (struct) 1.0 1.0 0.0 null null null null)
    (`self.StartHitstop` self)
    (`GameplayStatics.PlayWorldCameraShake` "/Game/Assets/VFX/CameraShake.CameraShake_C" _returnvalue 0.0 500.0)
    (`self.HitParticleEffects`)
    (bind _output_get (set `self.Health` (- (`self.Health`) `Damage Taken`)))
    (if (<= _output_get 0.0)
      (`/Engine/EditorBlueprintResources/StandardMacros.DoOnce` false
        (:`Completed`
          (`self.HurtHighlight`)
          (`self.PlayAnimMontage` "/Game/Assets/Animations/Enemies/AM_GolemDeath.AM_GolemDeath")
          (`GameplayStatics.PlaySound2D` null 1.0 1.0 0.0 null null)
          (set `self.Can Take Damage?` false)
          (`NiagaraFunctionLibrary.SpawnSystemAtLocation` "/Game/Assets/VFX/Enemy_VFX/NS_CorpseExplosionPurple.NS_CorpseExplosionPurple" _returnvalue_2)
          (`NiagaraFunctionLibrary.SpawnSystemAtLocation` "/Game/Assets/VFX/Enemy_VFX/NS_SmokePoof02.NS_SmokePoof02" _returnvalue_2)
          (`KismetSystemLibrary.Delay` 0.3)
          (bind _returnvalue_3 (`GameplayStatics.GetActorOfClass` "/Game/AI/WaveLogic/BP_WaveManager.BP_WaveManager_C"))
          (`/Engine/EditorBlueprintResources/StandardMacros.IsValid` _returnvalue_3
            (:`Is Valid`
              (`/Game/AI/WaveLogic/BP_WaveManager.SubtractFromNeeded` _returnvalue_3))
            (:`Is Not Valid`
              _))
          (`self.K2_DestroyActor`))))))

(event `/Game/Assets/BluePrints/Interfaces/BPIDamageRecievers.Knockback`
  (params (KnockbackSource :type "Vector Structure") (KnockbackValue :type "Float (double-precision)") (`Launch Value` :type "Float (double-precision)"))
  ;[1 1 1] Damage and knockback
  (if (not (`self.Is Immovable`))
    (`|ExecutionSequence`
      (:`then_0`
        (set `self.Launch Value` `Launch Value`)
        (set `self.Knockback Value` 0.0)
        (if (`self.First Hit?`)
          (bind _result (`/Engine/EditorBlueprintResources/StandardMacros.IncrementInt` (`self.Number Of Hits`) :!label _label)
            (:`  `
              (set `self.Number Of Hits` _result)
              (set `self.First Hit?` false)))
          (else
            (switch `int` (`self.Number Of Hits`)
              (:`0`
                (goto _label))
              (:`1`
                (`self.AddLaunch` 1.2))
              (:`2`
                (`self.AddLaunch` 1.5))
              (:`3`
                (`self.AddLaunch` 1.75))
              (:`4`
                (`self.AddLaunch` 2.5)
                (`self.AddKnockback` 30.0)))
            (bind _result_2 (`/Engine/EditorBlueprintResources/StandardMacros.IncrementInt` (`self.Number Of Hits`))
              (:`  `
                (set `self.Number Of Hits` _result_2)))))
        (`NavMovementComponent.StopActiveMovement` (`self.CharacterMovement`))
        (bind _applied_knockback (`self.Calculate KB Dir` KnockbackSource (`self.K2_GetActorLocation` self) (`self.Knockback Value`) (`self.Launch Value`)))
        (`self.LaunchCharacter` _applied_knockback true true)
        (if (>= (`self.Number Of Hits`) 5)
          (set `self.Number Of Hits` 0)))
      (:`then_1`
        (`KismetSystemLibrary.RetriggerableDelay` 1.5)
        (set `self.Number Of Hits` 0)))))

(event `SpawnExplosion`
  (bind _returnvalue (`KismetMathLibrary.RandomPointInBoundingBox` (`self.K2_GetActorLocation` (`self.As BP Main Character`)) (250.0 250.0 0.0)))
  (bind (_x _y _z) (`KismetMathLibrary.BreakVector3f` _returnvalue))
  (bind _outhit (`KismetSystemLibrary.LineTraceSingle` _returnvalue (`KismetMathLibrary.MakeVector` _x _y (- _z 2000.0)) "TraceTypeQuery1" false (`|MakeArray` (`self.As BP Main Character`) :!type "Actor Object Reference")))
  (`|SpawnActorFromClass` "/Game/Assets/BluePrints/Dummies/BP_IndicatorForAoe.BP_IndicatorForAoe_C" (`KismetMathLibrary.MakeTransform` (`.ImpactPoint` (`GameplayStatics.BreakHitResult` _outhit))) "Undefined" "OverrideRootScale" self null))

(fn `AddKnockback`
  (params (KnockbackBoost :type "Float (double-precision)")))

(fn `AddLaunch`
  (params (LaunchBoost :type "Float (double-precision)")))

(fn `EndHitstop`
  (set `self.CustomTimeDilation` 1.0))

(fn `StartHitstop`
  (params (Actor :type "Actor Object Reference"))
  (set `Actor.CustomTimeDilation` 0.0 Actor)
  (`KismetSystemLibrary.K2_SetTimer` null "EndHitstop" 0.1))

(fn `UserConstructionScript`
  (`parent.UserConstructionScript`))