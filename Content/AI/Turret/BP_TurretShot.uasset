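; BP_TurretShot is a turret projectile that homes in on the player character and damages it on contact.
; On BeginPlay it sets the player's capsule as the ProjectileMovement homing target and starts a timed self-destruct.
; Overlap of its Box with BP_MainCharacter calls TakeDamage with a fixed amount, then destroys the shot after a short delay.
; Overlaps with other actors are ignored.
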(event `self.ReceiveBeginPlay`
  (bind _projectilemovement (`self.ProjectileMovement`))
  (bind _asbp_main_character (cast `/Game/Assets/BluePrints/MainCharacter/BP_MainCharacter` (`GameplayStatics.GetPlayerCharacter` 0)))
  (bind _output_get (set `self.As BP Main Character` _asbp_main_character))
  (set `ProjectileMovementComponent.HomingTargetComponent` (`Character.CapsuleComponent` _output_get) _projectilemovement)
  (set `ProjectileMovementComponent.bIsHomingProjectile` true _projectilemovement)
  (`KismetSystemLibrary.Delay` 4.0)
  (`self.K2_DestroyActor`))

(event `self.ReceiveTick`
  (params (DeltaSeconds :type "Float (single-precision)")))

(event `self.Box.OnComponentBeginOverlap`
  (params (OverlappedComponent :type "PrimitiveComponent Object Reference") (OtherActor :type "Actor Object Reference") (OtherComp :type "PrimitiveComponent Object Reference") (OtherBodyIndex :type Integer) (bFromSweep :type Boolean) (SweepResult :type "HitResult Structure (by ref)"))
  (bind _asbp_main_character (cast `/Game/Assets/BluePrints/MainCharacter/BP_MainCharacter` OtherActor))
  (`/Game/Assets/BluePrints/Interfaces/BPIDamageRecievers.TakeDamage` _asbp_main_character 20.0)
  (`KismetSystemLibrary.Delay` 0.2)
  (`self.K2_DestroyActor`))

(fn `UserConstructionScript`)