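; Telegraph actor, named as a boss jump indicator, that shows a filling area marker and provides an explosion attack.
; On BeginPlay it creates dynamic materials for the circumference and area, then a timeline fills the area and destroys the actor when finished.
; Explosion, not called within this graph, spawns dark Niagara effects, sphere-traces to damage and knock back the player once, then destroys the actor.
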(event `self.ReceiveBeginPlay`
  (`|ExecutionSequence`
    (:`then_0`
      (bind _returnvalue (`DecalComponent.CreateDynamicMaterialInstance` (`self.Circum`)))
      (bind _output_get (set `self.CircumRef` _returnvalue))
      (`MaterialInstanceDynamic.SetScalarParameterValue` _output_get "Circum1Area0" 1.0))
    (:`then_1`
      (bind _returnvalue_2 (`DecalComponent.CreateDynamicMaterialInstance` (`self.Area`)))
      (bind _output_get_2 (set `self.AreaRef` _returnvalue_2))
      (`MaterialInstanceDynamic.SetScalarParameterValue` _output_get_2 "Circum1Area0" 0.0)
      (`MaterialInstanceDynamic.SetScalarParameterValue` _output_get_2 "AreaValue" 0.0))
    (:`then_2`
      (bind (_direction _fillvalue) (`Timeline|FillArea`)
        (:`Update`
          (`MaterialInstanceDynamic.SetScalarParameterValue` (`self.AreaRef`) "AreaValue" _fillvalue))
        (:`Finished`
          (`self.K2_DestroyActor`))))))

(fn `Explosion`
  (bind _returnvalue (`self.K2_GetActorLocation`))
  (`NiagaraFunctionLibrary.SpawnSystemAtLocation` "/Game/Assets/VFX/SpellVFX/NS_DarkExplosion.NS_DarkExplosion" _returnvalue)
  (bind _outhits (`KismetSystemLibrary.SphereTraceMultiForObjects` _returnvalue _returnvalue 250.0 (`self.Object Types`)))
  (for _array_element _outhits
    (bind _asbp_main_character (cast `/Game/Assets/BluePrints/MainCharacter/BP_MainCharacter` (`.HitActor` (`GameplayStatics.BreakHitResult` _array_element))))
    (`/Engine/EditorBlueprintResources/StandardMacros.IsValid` (`self.Player reference`)
      (:`Is Not Valid`
        (message `/Game/Assets/BluePrints/Interfaces/BPIDamageRecievers.TakeDamage` _asbp_main_character 20.0 0.0)
        (bind _output_get (set `self.Player reference` _asbp_main_character))
        (`/Game/Assets/BluePrints/MainCharacter/BP_MainCharacter.Knockback` _output_get (`self.K2_GetActorLocation` self) 1.0 1000.0))))
  (`ActorComponent.K2_DestroyComponent` (`self.Rockeffect`))
  (`self.K2_DestroyActor`))

(fn `UserConstructionScript`)