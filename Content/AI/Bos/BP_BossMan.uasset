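; Boss character that runs queued jump slam, charge, meteor rain, stomp and boulder throw attacks against the player.
; TranslateAttacks plays the Attacks array with recovery delays, then flags the boss stunned on the Blackboard for a vulnerable window.
; Timelines drive the spline leap and telegraphed charge, with indicator actors warning of impacts.
; Health thirds trigger phase transitions, BreakFloor1 destroys arena levels, and death stops AI and shows the end screen.
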(event `self.ChargeHitBox.OnComponentBeginOverlap`
  (params (OverlappedComponent :type "PrimitiveComponent Object Reference") (OtherActor :type "Actor Object Reference") (OtherComp :type "PrimitiveComponent Object Reference") (OtherBodyIndex :type Integer) (bFromSweep :type Boolean) (SweepResult :type "HitResult Structure (by ref)"))
  ;[1 0 0.5316] Charge HitBox Logic
  (if (not (== OtherActor self))
    (bind _asbp_main_character (cast `/Game/Assets/BluePrints/MainCharacter/BP_MainCharacter` OtherActor)
      (:`then`
        (`/Engine/EditorBlueprintResources/StandardMacros.DoOnce` false :!label _label
          (:`Completed`
            (`self.TakeDamage` _asbp_main_character 25.0)
            (`self.Knockback` _asbp_main_character (+ (`self.K2_GetActorLocation`) (* (`KismetMathLibrary.GetRightVector` (`self.K2_GetActorRotation`)) 200.0)) 500.0 500.0))))
      (:`CastFailed`
        (`self.StopCharging` :!label _label_2)
        (goto _label :!via `Reset`)))))

(event `ResetChargeHitBox`
  ;[1 0 0.5316] Charge HitBox Logic
  (goto _label_2))

(event `ShowChargeIndicator`
  (bind _returnvalue (`self.K2_GetActorLocation`))
  (bind _returnvalue_2 (`self.K2_GetActorLocation` (`self.MainCharacter`)))
  (bind (_returnvalue_roll _returnvalue_pitch _returnvalue_yaw) (`KismetMathLibrary.BreakRotator` (`KismetMathLibrary.FindLookAtRotation` _returnvalue _returnvalue_2)))
  ;[1 0 0.5316] Charge HitBox Logic
  (`self.LookAtPlayer`)
  (set `self.MyPosition` (`self.K2_GetActorLocation`))
  (bind _output_get (set `self.DirectionToPlayer` (`KismetMathLibrary.Normal` (- (`self.K2_GetActorLocation` (`self.MainCharacter`)) (`self.K2_GetActorLocation`)))))
  (bind (_returnvalue_x _returnvalue_y) (`KismetMathLibrary.BreakVector` (* _output_get 1000.0)))
  (set `self.ChargeDistance` (+ (`KismetMathLibrary.MakeVector` _returnvalue_x _returnvalue_y) _returnvalue_2))
  (bind _returnvalue_3 (`|SpawnActorFromClass` "/Game/AI/Bos/BP_IndicatorCharge.BP_IndicatorCharge_C" (`KismetMathLibrary.MakeTransform` (+ (* (- (`self.ChargeDistance`) _returnvalue) 0.5) _returnvalue) (`KismetMathLibrary.MakeRotator` _returnvalue_roll 0.0 _returnvalue_yaw)) "Undefined" "OverrideRootScale" null null))
  (`/Game/AI/Bos/BP_IndicatorCharge.SetScaleForAOE` _returnvalue_3 (`KismetMathLibrary.VSize` (* (- (`self.ChargeDistance`) (`self.MyPosition`)) 0.5)))
  (bind (_direction _fillvalue) (`Timeline|ChargeUp` :!via `PlayFromStart`)
    (:`Update`
      (`/Game/AI/Bos/BP_IndicatorCharge.SetOpacity` _returnvalue_3 _fillvalue))
    (:`Finished`
      (`self.Charge`)
      (`self.K2_DestroyActor` _returnvalue_3))))

(event `Charge`
  (bind (_chargedistance_x _chargedistance_y) (`KismetMathLibrary.BreakVector` (`self.ChargeDistance`)))
  (bind (_myposition_x _myposition_y _myposition_z) (`KismetMathLibrary.BreakVector` (`self.MyPosition`)))
  ;[1 0 0.5316] Charge HitBox Logic
  (set `PrimitiveComponent.bGenerateOverlapEvents` true (`self.ChargeHitBox`))
  (bind (_direction _move_to_destination) (`Timeline|Timeline` :!via `PlayFromStart` :!label _label_3)
    (:`Update`
      (`self.K2_SetActorLocation` (`KismetMathLibrary.VLerp` (`self.MyPosition`) (`KismetMathLibrary.MakeVector` _chargedistance_x _chargedistance_y _myposition_z) _move_to_destination)))
    (:`Finished`
      (set `PrimitiveComponent.bGenerateOverlapEvents` false (`self.ChargeHitBox`))
      (`self.ResetChargeHitBox`))))

(event `StopCharging`
  ;[1 0 0.5316] Charge HitBox Logic
  (`|ExecutionSequence`
    (:`then_0`
      (set `self.IsDashing?` false)
      (set `PrimitiveComponent.bGenerateOverlapEvents` false (`self.ChargeHitBox`))
      (goto _label_3 :!via `Stop`))))

(event `JumpAttack`
  (bind _returnvalue (`self.K2_GetActorLocation`))
  (bind _output (`|GetArrayItem` (`self.JumpTrajectoryPoint`) 2))
  ;[1 0.1754 0.5948] Jump Logci
  ;;[1 1 1] Make Trajectory for jump
  (`KismetArrayLibrary.Array_Add` (`self.JumpTrajectoryPoint`) _returnvalue)
  (`KismetArrayLibrary.Array_Add` (`self.JumpTrajectoryPoint`) (+ (+ (* (- (`self.K2_GetActorLocation` (`self.MainCharacter`)) _returnvalue) 0.5) _returnvalue) (0.0 0.0 1000.0)))
  (`KismetArrayLibrary.Array_Add` (`self.JumpTrajectoryPoint`) (`self.K2_GetActorLocation` (`self.MainCharacter`)))
  (`SplineComponent.SetSplinePoints` (`self.JumpTrajectory`) (`self.JumpTrajectoryPoint`) "Local" true)
  ;;[1 1 1] Set Boss location
  (bind (_direction _timetodestination) (`Timeline|JumpSlam` :!via `PlayFromStart`)
    (:`Update`
      (`self.K2_SetActorLocation` (`SplineComponent.GetLocationAtTime` (`self.JumpTrajectory`) _timetodestination "Local" false)))
    (:`Finished`
      (`|ExecutionSequence`
        (:`then_0`
          (`KismetArrayLibrary.Array_Clear` (`self.JumpTrajectoryPoint`))
          (`GameplayStatics.PlayWorldCameraShake` "/Game/Assets/VFX/CameraShakeRupture.CameraShakeRupture_C" (`self.K2_GetActorLocation`) 1000.0 10000.0)
          (`self.AoeDamage` 600.0 400.0 2000.0)
          (`NiagaraFunctionLibrary.SpawnSystemAtLocation` "/Game/Assets/VFX/MovementVFX/NS_RuptureJumpAttack.NS_RuptureJumpAttack" (`SceneComponent.K2_GetComponentLocation` (`self.RefFeet`)) (struct) (2.0 2.0 2.0)))))
    (:`SpawnIndicator`
      ;;[1 1 1] Spawn Indicator at impact point
      (bind _outhit (`KismetSystemLibrary.LineTraceSingleForObjects` _output (+ (* (`KismetMathLibrary.Vector_Down`) 400.0) _output) (`self.Objecttypes`) false (`|MakeArray` (`self.MainCharacter`) :!type "Actor Object Reference")))
      (`|SpawnActorFromClass` "/Game/AI/Bos/BP_BossIndicatorForJump.BP_BossIndicatorForJump_C" (`KismetMathLibrary.MakeTransform` (`.ImpactPoint` (`GameplayStatics.BreakHitResult` _outhit))) "Undefined" "OverrideRootScale" null null))
    (:`SetSlamAnim`
      (set `self.IsJumping?` false))))

(event `StartChargeAttack`
  ;[1 0.5019 0.416] Call For Attacks
  (set `self.IsDashing?` true)
  (`GameplayStatics.PlaySound2D` "/Game/SoundFX/MetaSounds/Implemented/MS_BossLaughCharge.MS_BossLaughCharge" 1.0 1.0 0.0 null null))

(event `StartJumpAttack`
  ;[1 0.5019 0.416] Call For Attacks
  (`self.LookAtPlayer`)
  (set `self.IsJumping?` true)
  (`GameplayStatics.PlaySound2D` "/Game/SoundFX/MetaSounds/Implemented/MS_BossLaughJump.MS_BossLaughJump" 1.0 1.0 0.0 null null))

(event `StartMeteorRain`
  ;[1 0.5019 0.416] Call For Attacks
  (set `self.MeteorRain?` true))

(event `StartThrow`
  ;[1 0.5019 0.416] Call For Attacks
  (set `self.IsThrowing?` true)
  (`Timeline|LookAtPlayerTimeline` :!via `PlayFromStart`
    (:`Update`
      (`self.LookAtPlayer`))))

(event `StartStomp`
  ;[1 0.5019 0.416] Call For Attacks
  (set `self.IsStomping?` true)
  (`|SpawnActorFromClass` "/Game/AI/Bos/BP_BossIndicatorForStomp.BP_BossIndicatorForStomp_C" (`KismetMathLibrary.MakeTransform` (`SceneComponent.K2_GetComponentLocation` (`self.RefFeet`))) "Undefined" "OverrideRootScale" null null)
  (`KismetSystemLibrary.Delay` 0.2)
  (set `self.IsStomping?` false))

(event `self.ReceiveBeginPlay`
  ;[1 0.5879 0] Begin Pay
  (`|ExecutionSequence`
    (:`then_0`
      (bind _asbp_main_character (cast `/Game/Assets/BluePrints/MainCharacter/BP_MainCharacter` (`GameplayStatics.GetPlayerCharacter` 0)))
      (set `self.MainCharacter` _asbp_main_character)
      (set `PrimitiveComponent.bGenerateOverlapEvents` false (`self.ChargeHitBox`))
      (`SceneComponent.K2_DetachFromComponent` (`self.JumpTrajectory`) "KeepRelative" "KeepRelative" "KeepRelative" true)
      (`self.Walking Timer`))
    (:`then_1`
      (bind _returnvalue (`|CreateWidget` "/Game/Assets/UI/HUD_Widgets/WBP_HealthbarBossman.WBP_HealthbarBossman_C" (`GameplayStatics.GetPlayerController` 0)))
      (bind _output_get (set `self.BossHealthUI` _returnvalue))
      (`UserWidget.AddToViewport` _output_get 0))))

(event `Meteor rain`
  ;[0.2014 0 1] Meteor
  (bind _locations (`self.GetMeteorLocations`))
  (for _array_element _locations
    (bind _outhit (`KismetSystemLibrary.LineTraceSingle` (+ _array_element (0.0 0.0 300.0)) (+ _array_element (* (`KismetMathLibrary.Vector_Down`) 400.0)) "TraceTypeQuery1" false (`|MakeArray` (`self.MainCharacter`) :!type "Actor Object Reference")))
    (`|SpawnActorFromClass` "/Game/AI/Bos/BP_BossIndicatorForExplosion.BP_BossIndicatorForExplosion_C" (`KismetMathLibrary.MakeTransform` (`.ImpactPoint` (`GameplayStatics.BreakHitResult` _outhit))) "Undefined" "OverrideRootScale" null null))
  (`KismetSystemLibrary.Delay` 1.5)
  (set `self.MeteorRain?` false)
  (`GameplayStatics.PlayWorldCameraShake` "/Game/Assets/VFX/CameraShakeRupture.CameraShakeRupture_C" (`self.K2_GetActorLocation`) 10000.0 10000.0))

(event `Walking Timer`
  ;[0.4812 0.3636 1] Walking Timer
  (set `self.IsWalking?` true)
  (`KismetSystemLibrary.Delay` 2.0)
  (set `self.IsWalking?` false))

(event `TranslateAttacks`
  (bind _attacks (`self.Attacks`))
  ;[1 0 0] Attack Logci
  (set `self.IsAttacking?` true)
  (bind _output_get (set `self.Tracker` 0))
  (if (<= _output_get (- (`KismetArrayLibrary.Array_Length` _attacks) 1)) :!label _label_4
    ;;[1 1 1] Comment
    (if (not (`self.Is Dead?`))
      (switch `int` (`|GetArrayItem` _attacks (`self.Tracker`))
        (:`0`
          (`self.StartJumpAttack`)
          (`KismetSystemLibrary.Delay` (`self.RecJump`)))
        (:`1`
          (`self.StartChargeAttack`)
          (`KismetSystemLibrary.Delay` (`self.RecCharge`)))
        (:`2`
          (`self.StartMeteorRain`)
          (`KismetSystemLibrary.Delay` (`self.RecMeteor`)))
        (:`3`
          (`self.StartStomp`)
          (`KismetSystemLibrary.Delay` (`self.StompRecovery`)))
        (:`4`
          (`self.StartThrow`)
          (`KismetSystemLibrary.Delay` (`self.ThrowRecovery`))))
      (set `self.Tracker` (+ (`self.Tracker`) 1))
      (goto _label_4))
    (else
      (`KismetArrayLibrary.Array_Clear` (`self.Attacks`))
      (`|ExecutionSequence`
        (:`then_0`
          (bind _output_get_2 (set `self.IsUnderRecovery` true))
          (`BlackboardComponent.SetValueAsBool` (`AIBlueprintHelperLibrary.GetBlackboard` null) "IsStunned?" _output_get_2))
        (:`then_1`
          (`KismetSystemLibrary.Delay` (`self.VulnerableTimer`))
          (if (not (`self.Is Dead?`))
            (bind _output_get_3 (set `self.IsUnderRecovery` false))
            (`BlackboardComponent.SetValueAsBool` (`AIBlueprintHelperLibrary.GetBlackboard` null) "IsStunned?" _output_get_3)
            (set `self.IsWalking?` true)
            (`KismetSystemLibrary.Delay` 2.0)
            (set `self.IsWalking?` false)
            (set `self.IsAttacking?` false)))))))

(event `Stomp`
  ;[0.199 1 0.1343] Stomp Logic
  (`self.AoeDamage` 700.0 2000.0 1000.0)
  (`GameplayStatics.PlayWorldCameraShake` "/Game/Assets/VFX/CameraShakeRupture.CameraShakeRupture_C" (`self.K2_GetActorLocation`) 2000.0 2000.0)
  (`NiagaraFunctionLibrary.SpawnSystemAtLocation` "/Game/Assets/VFX/MovementVFX/NS_RuptureJumpAttack.NS_RuptureJumpAttack" (`SceneComponent.K2_GetComponentLocation` (`self.RefFeet`)) (struct) (2.0 2.0 1.0)))

(event `BoulderThrow`
  (bind _returnvalue (`SceneComponent.K2_GetComponentLocation` (`self.BoulderTossRef`)))
  (bind (_returnvalue_roll _returnvalue_pitch _returnvalue_yaw) (`KismetMathLibrary.BreakRotator` (`KismetMathLibrary.FindLookAtRotation` _returnvalue (`self.K2_GetActorLocation` (`self.MainCharacter`)))))
  ;[1 0.836 0] throw Boulder
  (`|SpawnActorFromClass` "/Game/AI/Bos/BP_BoulderToss.BP_BoulderToss_C" (`KismetMathLibrary.MakeTransform` _returnvalue (`KismetMathLibrary.MakeRotator` _returnvalue_roll 0.0 _returnvalue_yaw)) "Undefined" "OverrideRootScale" self null)
  (`GameplayStatics.PlaySound2D` "/Game/SoundFX/MetaSounds/Implemented/MS_RockThrowWoosh.MS_RockThrowWoosh" 1.0 1.0 0.0 null null)
  (set `self.IsThrowing?` false))

(event `self.TakeDamage`
  (params (`Damage Taken` :type "Float (double-precision)"))
  ;[0.05119 1 0] DamageLogic
  (if (not (`self.Is Dead?`))
    (`self.HurtFeedBack`)
    (set `self.Health` (- (`self.Health`) `Damage Taken`))
    (`self.UpdatePhase`)
    (`|ExecutionSequence`
      (:`then_0`
        (`/Game/Assets/BluePrints/MainCharacter/BPC_HealthSystemBoss.DecreaseHealth` (`self.BPC_HealthSystemBoss`) `Damage Taken`)
        (if (`self.IsUnderRecovery`)
          (set `self.IsDamaged?` true)
          (`KismetSystemLibrary.Delay` 0.5)
          (set `self.IsDamaged?` false)))
      (:`then_1`
        (if (<= (`self.Health`) 0.0)
          (set `self.Is Dead?` true)
          (`BrainComponent.StopLogic` (`AIController.BrainComponent` (`AIBlueprintHelperLibrary.GetAIController` self)) "")
          (`SkeletalMeshComponent.PlayAnimation` (`self.Mesh`) "/Game/AI/Bos/Anim/Boss_death.Boss_death" false)
          (`KismetArrayLibrary.Array_Clear` (`self.Attacks`))
          (`KismetSystemLibrary.Delay` 5.0)
          (bind _returnvalue (`|CreateWidget` "/Game/Assets/UI/Menu_Widgets/WBP_Screen_End.WBP_Screen_End_C" (`GameplayStatics.GetPlayerController` 0)))
          (`UserWidget.AddToViewport` _returnvalue 0))))))

(event `StunnPlayer`
  (bind _charactermovement (`Character.CharacterMovement` (`self.MainCharacter`)))
  ;[1 1 1] Budget Stun
  (`CharacterMovementComponent.DisableMovement` _charactermovement)
  (`KismetSystemLibrary.Delay` 1.5)
  (`CharacterMovementComponent.SetMovementMode` _charactermovement "MOVE_Walking" 0))

(event `HurtFeedBack`
  (bind _mesh (`self.Mesh`))
  (bind _mesh_2 (`self.Mesh`))
  ;[0.4302 0.272 0.272] Swap To Hurt Material
  (`PrimitiveComponent.SetMaterial` (`self.Mesh`) 0 "/Game/AI/Bos/Textures/NewTextures/MI_Hurt_Main.MI_Hurt_Main")
  (`PrimitiveComponent.SetMaterial` _mesh_2 1 "/Game/AI/Bos/Textures/NewTextures/MI_ShoulderGuardHurt.MI_ShoulderGuardHurt")
  (`PrimitiveComponent.SetMaterial` _mesh_2 3 "/Game/AI/Bos/Textures/NewTextures/MI_TankHurt.MI_TankHurt")
  (`PrimitiveComponent.SetMaterial` _mesh_2 4 "/Game/AI/Bos/Textures/NewTextures/MI_WeaponHurt.MI_WeaponHurt")
  (`KismetSystemLibrary.Delay` 0.2)
  (`PrimitiveComponent.SetMaterial` (`self.Mesh`) 0 "/Game/AI/Bos/Textures/NewTextures/MI_BossColor.MI_BossColor")
  (`PrimitiveComponent.SetMaterial` _mesh 1 "/Game/AI/Bos/Textures/NewTextures/MI_ShoulderGuard.MI_ShoulderGuard")
  (`PrimitiveComponent.SetMaterial` _mesh 3 "/Game/AI/Bos/Textures/NewTextures/MI_Tank.MI_Tank")
  (`PrimitiveComponent.SetMaterial` _mesh 4 "/Game/AI/Bos/Textures/NewTextures/MI_Weapon.MI_Weapon"))

(event `Phase2Transition`
  (`KismetArrayLibrary.Array_Clear` (`self.Attacks`) :!label _label_5)
  (`self.PlayAnimMontage` "/Game/AI/Bos/Anim/Montages/Montage_Stomp.Montage_Stomp" 2.0)
  (`KismetSystemLibrary.Delay` 0.7)
  (`self.Knockback` (`self.MainCharacter`) (`self.K2_GetActorLocation`) 10000.0 100.0)
  (`self.PlayAnimMontage` "/Game/AI/Bos/Anim/Montages/Montage_Stomp.Montage_Stomp" 2.0)
  (`KismetSystemLibrary.Delay` 2.0)
  (`self.PlayAnimMontage` "/Game/AI/Bos/Anim/Montages/Montage_BreakGround.Montage_BreakGround"))

(event `BreakFloor1`
  (`GameplayStatics.PlayWorldCameraShake` "/Game/Assets/VFX/GroundBreakShake.GroundBreakShake_C" (`self.K2_GetActorLocation`) 100.0 10000.0)
  (`/Engine/EditorBlueprintResources/StandardMacros.FlipFlop`
    (:`A`
      (`KismetSystemLibrary.Delay` 1.0)
      (for _array_element (`self.FirstLevel`)
        (`self.K2_DestroyActor` _array_element)
        (`KismetSystemLibrary.Delay` 2.0 :!label _label_6)
        (`BlackboardComponent.SetValueAsBool` (`AIBlueprintHelperLibrary.GetBlackboard` null) "Transitioning?" false)))
    (:`B`
      (for _array_element_2 (`self.SecondLevel`)
        (`self.K2_DestroyActor` _array_element_2)
        (goto _label_6)))))

(event `Phase3Transition`
  (goto _label_5))

(fn `AddTOAttacks`
  (params (Attacks :type "Array of Integer"))
  (`KismetArrayLibrary.Array_Clear` (`self.Attacks`))
  (set `self.Attacks` Attacks))

(fn `AoeDamage`
  (params (Radius :type "Float (double-precision)") (Knockback :type "Float (double-precision)") (Launch :type "Float (double-precision)"))
  (bind _returnvalue (`self.K2_GetActorLocation`))
  (bind _outhits (`KismetSystemLibrary.SphereTraceMulti` _returnvalue _returnvalue Radius "TraceTypeQuery1"))
  (for _array_element _outhits
    (bind (_bblockinghit _binitialoverlap _time _distance _location _impactpoint _normal _impactnormal _physmat _hitactor) (`GameplayStatics.BreakHitResult` _array_element))
    (if (not (== self _hitactor))
      (bind _asbpidamage_recievers (cast `/Game/Assets/BluePrints/Interfaces/BPIDamageRecievers` _hitactor))
      (if (not (`KismetArrayLibrary.Array_Contains` (`self.Damaged`) _asbpidamage_recievers))
        (`self.TakeDamage` _asbpidamage_recievers 25.0)
        (`self.Knockback` _asbpidamage_recievers (`self.K2_GetActorLocation`) Knockback Launch)
        (`KismetArrayLibrary.Array_Add` (`self.Damaged`) _asbpidamage_recievers))))
  (`KismetArrayLibrary.Array_Clear` (`self.Damaged`)))

(fn `Check Conditions`
  (returns (`IsDoing?` :type Boolean))
  (locals (ConditionIsMet :type Boolean :default true))
  (if (`self.IsDashing?`)
    (set `local.ConditionIsMet` false)
    (elif (`self.IsJumping?`)
      (set `local.ConditionIsMet` false)
      (elif (`self.MeteorRain?`)
        (set `local.ConditionIsMet` false))))
  (return (`local.ConditionIsMet`)))

(fn `GetMeteorLocations`
  (returns (Locations :type "Array of Vector Structure"))
  (bind _capsulecomponent (`Character.CapsuleComponent` (`self.MainCharacter`)))
  (bind _returnvalue (`SceneComponent.GetRightVector` _capsulecomponent))
  (bind _output_get (set `self.Forward Offset` (+ (* (`SceneComponent.GetForwardVector` _capsulecomponent) (`self.HitDistanceForward`)) (`self.K2_GetActorLocation` (`self.MainCharacter`)))))
  (return (`|MakeArray` (`self.K2_GetActorLocation` (`self.MainCharacter`)) (+ _output_get (* _returnvalue (`self.HitDistance Side`))) (+ _output_get (* (`KismetMathLibrary.NegateVector` _returnvalue) (`self.HitDistance Side`))) (+ (`self.K2_GetActorLocation` (`self.MainCharacter`)) (* (`KismetMathLibrary.NegateVector` (`SceneComponent.GetForwardVector` (`Character.CapsuleComponent` (`self.MainCharacter`)))) (`self.HitDistanceForward`))))))

(fn `LookAtPlayer`
  (bind (_returnvalue_roll _returnvalue_pitch _returnvalue_yaw) (`KismetMathLibrary.BreakRotator` (`KismetMathLibrary.FindLookAtRotation` (`self.K2_GetActorLocation`) (`self.K2_GetActorLocation` (`self.MainCharacter`)))))
  (`self.K2_SetActorRotation` (`KismetMathLibrary.MakeRotator` _returnvalue_roll 0.0 _returnvalue_yaw)))

(fn `SetPhaseVariables`
  (params (Phase2 :type Boolean) (Phase3 :type Boolean))
  (bind _returnvalue (`AIBlueprintHelperLibrary.GetBlackboard` null))
  (`BlackboardComponent.SetValueAsBool` _returnvalue "Phase2" Phase2)
  (`BlackboardComponent.SetValueAsBool` _returnvalue "Phase3" Phase3))

(fn `UpdatePhase`
  (if (`self.Phase3`)
    _
    (elif (`self.IsPhase2?`)
      (if (`self.Phase3`)
        _
        (elif (<= (`self.Health`) (/ (`self.MaxHealth`) 3.0))
          (bind _output_get (set `self.IsPhase2?` false))
          (bind _output_get_2 (set `self.Phase3` true))
          (`self.SetPhaseVariables` _output_get _output_get_2)
          (set `self.VulnerableTimer` 2.0)
          (`self.Phase3Transition`)
          (`BlackboardComponent.SetValueAsBool` (`AIBlueprintHelperLibrary.GetBlackboard` null) "Transitioning?" true :!label _label)))
      (elif (<= (`self.Health`) (* (/ (`self.MaxHealth`) 3.0) 2.0))
        (set `self.IsPhase2?` true)
        (`self.SetPhaseVariables` true)
        (`self.Phase2Transition`)
        (goto _label)))))

(fn `UserConstructionScript`
  (set `self.MaxHealth` (`self.Health`)))