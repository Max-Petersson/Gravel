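; BP_BoulderToss is a boulder actor for the boss fight that damages and stuns the player on contact.
; On BeginPlay it caches its owner as BP_BossMan.
; Its Box overlap ignores itself and its owner, applies fixed damage to BP_MainCharacter and calls the boss's StunnPlayer.
; Any other valid overlap, player or not, spawns a Niagara impact effect and destroys the boulder.
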(event `self.ReceiveBeginPlay`
  (bind _asbp_boss_man (cast `/Game/AI/Bos/BP_BossMan` (`self.GetOwner`)))
  (set `self.As BP Boss Man` _asbp_boss_man))

(event `self.Box.OnComponentBeginOverlap`
  (params (OverlappedComponent :type "PrimitiveComponent Object Reference") (OtherActor :type "Actor Object Reference") (OtherComp :type "PrimitiveComponent Object Reference") (OtherBodyIndex :type Integer) (bFromSweep :type Boolean) (SweepResult :type "HitResult Structure (by ref)"))
  (if (== OtherActor self)
    _
    (elif (not (== OtherActor (`self.GetOwner`)))
      (bind _asbp_main_character (cast `/Game/Assets/BluePrints/MainCharacter/BP_MainCharacter` OtherActor)
        (:`then`
          (`/Game/Assets/BluePrints/MainCharacter/BP_MainCharacter.TakeDamage` _asbp_main_character 15.0)
          (`/Game/AI/Bos/BP_BossMan.StunnPlayer` (`self.As BP Boss Man`))
          (`NiagaraFunctionLibrary.SpawnSystemAtLocation` "/Game/Assets/VFX/SpellVFX/NS_BoulderImpact.NS_BoulderImpact" (`self.K2_GetActorLocation`))
          (`self.K2_DestroyActor`))
        (:`CastFailed`
          (`NiagaraFunctionLibrary.SpawnSystemAtLocation` "/Game/Assets/VFX/SpellVFX/NS_BoulderImpact.NS_BoulderImpact" (`self.K2_GetActorLocation`))
          (`self.K2_DestroyActor`))))))

(fn `UserConstructionScript`)