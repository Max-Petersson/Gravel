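; Wave manager that runs a kill-gated wave encounter, tracking progress on an on-screen wave counter widget.
; External calls raise or lower the kills-needed count; reaching zero, or calling StartWaves, triggers CallSpawnNewWave and advances the wave with a camera shake.
; Once waves run out, it marks the HUD finished and, once only, plays a falling-wall sound and destroys the door components.
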(event `self.ReceiveBeginPlay`
  (bind _returnvalue (`|CreateWidget` "/Game/Assets/UI/HUD_Widgets/WBP_WaveCounter.WBP_WaveCounter_C" (`GameplayStatics.GetPlayerController` 0)))
  (bind _output_get (set `self.WaveHUD_ref` _returnvalue))
  (`UserWidget.AddToViewport` _output_get 0)
  (`/Game/Assets/UI/HUD_Widgets/WBP_WaveCounter.CreateWaveText` _output_get (`self.CurrentWave`) (`self.MaxWaves`)))

(event `AddToNeeded`
  (bind _result (`/Engine/EditorBlueprintResources/StandardMacros.IncrementInt` (`self.KillsNeeded`))
    (:`  `
      (set `self.KillsNeeded` _result))))

(event `SubtractFromNeeded`
  (bind _door (`self.Door`))
  (bind _result (`/Engine/EditorBlueprintResources/StandardMacros.DecrementInt` (`self.KillsNeeded`))
    (:`  `
      (bind _output_get (set `self.KillsNeeded` _result))
      (if (<= _output_get 0)
        (`self.SpawnNewWave` (- (`self.CurrentWave`) 1) :!label _label)
        (if (> (+ (`self.CurrentWave`) 1) (`self.MaxWaves`))
          ;[1 1 1] Waves Cleared
          (`/Game/Assets/UI/HUD_Widgets/WBP_WaveCounter.FinishAllWaves` (`self.WaveHUD_ref`))
          (`/Engine/EditorBlueprintResources/StandardMacros.DoOnce` false
            (:`Completed`
              (`GameplayStatics.PlaySound2D` "/Game/SoundFX/MetaSounds/Implemented/MS_StoneWallFalling.MS_StoneWallFalling" 1.2 1.0 0.0 null null)
              (`/Engine/EditorBlueprintResources/StandardMacros.IsValid` _door
                (:`Is Valid`
                  (`ActorComponent.K2_DestroyComponent` _door)
                  (`ActorComponent.K2_DestroyComponent` (`self.StaticMesh7`))
                  (`ActorComponent.K2_DestroyComponent` (`self.StaticMesh3`))
                  (`ActorComponent.K2_DestroyComponent` (`self.StaticMesh`))
                  (`ActorComponent.K2_DestroyComponent` (`self.StaticMesh2`))
                  (`ActorComponent.K2_DestroyComponent` (`self.StaticMesh4`))
                  (`ActorComponent.K2_DestroyComponent` (`self.Box`))
                  (`ActorComponent.K2_DestroyComponent` (`self.StaticMesh1`))
                  (`ActorComponent.K2_DestroyComponent` (`self.StaticMesh5`))
                  (`ActorComponent.K2_DestroyComponent` (`self.StaticMesh6`))))))
          (else
            ;[1 1 1] Play the new wave
            (bind _output_get_2 (set `self.CurrentWave` (+ 1 (`self.CurrentWave`))))
            (`/Game/Assets/UI/HUD_Widgets/WBP_WaveCounter.UpdateCurrentWave` (`self.WaveHUD_ref`) _output_get_2)
            (`PlayerCameraManager.StartCameraShake` :`self` (`PlayerController.PlayerCameraManager` (`GameplayStatics.GetPlayerController` 0)) :`ShakeClass` "/Game/Assets/VFX/CameraWaveShake.CameraWaveShake_C" :`Scale` 0.4)))))))

(event `StartWaves`
  (goto _label))

(fn `UserConstructionScript`)