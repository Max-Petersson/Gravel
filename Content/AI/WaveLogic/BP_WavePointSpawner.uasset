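; Wave spawner actor that processes per-wave counts of three enemy types (FS, Brutes, Turrets) within a box volume sized by SpawnArea.
; On BeginPlay, NextWave loops through each count, firing debug-drawn downward line traces at randomized points.
; After each count it advances WhatToSpawn, incrementing CurrentWave when that index wraps.
; Spawning is unfinished: trace results are unused and the SpawnActor node is disconnected.
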(event `self.ReceiveBeginPlay`
  (`self.NextWave`))

(event `IndexOutOfRange`
  (bind _output_get (set `self.What To Spawn` (+ (`self.What To Spawn`) 1) :!label _label))
  (if (== _output_get 3)
    (set `self.What To Spawn` 0)
    (set `self.CurrentWave` (+ 1 (`self.CurrentWave`)))))

(event `NextWave`
  (bind (_returnvalue_x _returnvalue_y) (`KismetMathLibrary.BreakVector` (`self.K2_GetActorLocation`)))
  (bind (_returnvalue_x_2 _returnvalue_y_2 _returnvalue_z) (`KismetMathLibrary.BreakVector` (`self.K2_GetActorLocation`)))
  (bind (_returnvalue_x_3 _returnvalue_y_3 _returnvalue_z_2) (`KismetMathLibrary.BreakVector` (`self.K2_GetActorLocation`)))
  (bind (_spawnarea_x _spawnarea_y) (`KismetMathLibrary.BreakVector` (`self.SpawnArea`)))
  (bind (_spawnarea_x_2 _spawnarea_y_2 _spawnarea_z) (`KismetMathLibrary.BreakVector` (`self.SpawnArea`)))
  (bind _returnvalue (+ (`KismetMathLibrary.RandomFloatInRange` (* (/ _spawnarea_y 2.0) -1.0) _spawnarea_y) _returnvalue_y))
  (bind _returnvalue_2 (+ (`KismetMathLibrary.RandomFloatInRange` (* (/ _spawnarea_x 2.0) -1.0) _spawnarea_x) _returnvalue_x))
  (`|ExecutionSequence`
    (:`then_0`
      (if (`KismetArrayLibrary.Array_IsValidIndex` (`self.Amount FS`) (`self.CurrentWave`))
        (set `self.Tracker` (`|GetArrayItem` (`self.Amount FS`) (`self.CurrentWave`)))
        (bind _output_get (set `self.Tracker` (- (`self.Tracker`) 1) :!label _label_2))
        (if (< _output_get 0)
          (goto _label)
          (else
            (`KismetSystemLibrary.LineTraceSingle` :`Start` (`KismetMathLibrary.MakeVector` _returnvalue_2 _returnvalue _returnvalue_z_2) :`End` (+ (* (`KismetMathLibrary.Vector_Down`) (/ _spawnarea_z 0.5)) (`KismetMathLibrary.MakeVector` _returnvalue_2 _returnvalue _returnvalue_z)) :`TraceChannel` "TraceTypeQuery1" :`DrawDebugType` "ForDuration")
            (goto _label_2)))
        (else
          _)))
    (:`then_1`
      (if (`KismetArrayLibrary.Array_IsValidIndex` (`self.Amount Brutes`) (`self.CurrentWave`))
        (set `self.Tracker` (`|GetArrayItem` (`self.Amount Brutes`) (`self.CurrentWave`)))
        (goto _label_2)
        (else
          _)))
    (:`then_2`
      (if (`KismetArrayLibrary.Array_IsValidIndex` (`self.Amount Turrets`) (`self.CurrentWave`))
        (set `self.Tracker` (`|GetArrayItem` (`self.Amount Turrets`) (`self.CurrentWave`)))
        (goto _label_2)
        (else
          _))))
  (`self.IndexOutOfRange`))

(fn `UserConstructionScript`
  (`BoxComponent.SetBoxExtent` (`self.Box`) (`self.SpawnArea`) true))