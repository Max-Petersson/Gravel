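; Golem footsoldier enemy that rises from the ground, registers with BP_WaveManager, then runs its behavior tree against the player.
; Light and heavy attacks use a capsule trace to damage and knock back the player, gated to one hit per swing.
; Incoming knockback escalates launch strength over a timed hit counter, unless attacking has made it immovable.
; Damage triggers flash, sound and shake; death plays effects, decrements the wave count and usually drops an orb.
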(event `HurtHighlight`
  (bind _mesh (`self.Mesh`))
  ;[1 1 1] Hurt Highlight
  (`PrimitiveComponent.SetMaterial` _mesh 0 "/Game/Assets/Materials/Enemies/M_HurtHighlight.M_HurtHighlight")
  (`KismetSystemLibrary.Delay` 0.2)
  (`PrimitiveComponent.SetMaterial` _mesh 0 "/Game/Assets/Meshes/Enemies/Golem/Golem_material1.Golem_material1"))

(event `/Game/AI/EnemyFootsoldier/BPI_AICombat.AIMeleeAttack`
  ;[1 0.1195 0.1195] AI Melee
  (set `self.Is Immovable` true)
  (`self.PlayAnimMontage` "/Game/Assets/Animations/Enemies/AM_GolemLightAttack.AM_GolemLightAttack")
  (`GameplayStatics.SetGlobalTimeDilation` 1.0 :!label _label)
  (set `self.Can damage?` true))

(event `AI Light Attack Trace`
  ;[1 0.1195 0.1195] AI Attack Sphere Trace Footsoldier
  (`self.GolemAttack` 10.0 450.0 100.0))

(event `/Game/Assets/BluePrints/Interfaces/BPIDamageRecievers.TakeDamage`
  (params (`Damage Taken` :type "Float (double-precision)") (PoiseDamage :type "Float (double-precision)"))
  (bind _mesh (`self.Mesh`))
  (bind _returnvalue (`self.K2_GetActorLocation` self))
  (bind _returnvalue_2 (`SceneComponent.K2_GetComponentLocation` (`self.Mesh`)))
  (bind _returnvalue_3 (`KismetMathLibrary.Conv_VectorToTransform` _returnvalue_2))
  ;[1 1 1] Damage and knockback
  (if (`self.CanTakeDamage?`)
    (`self.HurtHighlight`)
    (`/Engine/EditorBlueprintResources/StandardMacros.FlipFlop`
      (:`A`
        (`SkeletalMeshComponent.PlayAnimation` _mesh "/Game/Assets/Animations/Enemies/AM_GolemTakeDamageLeft.AM_GolemTakeDamageLeft" false))
      (:`B`
        (`SkeletalMeshComponent.PlayAnimation` _mesh "/Game/Assets/Animations/Enemies/AM_GolemTakeDamageRight.AM_GolemTakeDamageRight" false)))
    (`GameplayStatics.PlaySoundAtLocation` "/Game/SoundFX/EnemyHit.EnemyHit" _returnvalue (struct) 1.0 1.0 0.0 null null null null)
    (`GameplayStatics.PlayWorldCameraShake` "/Game/Assets/VFX/CameraShake.CameraShake_C" _returnvalue 0.0 1000.0)
    (bind _output_get (set `self.Health` (- (`self.Health`) `Damage Taken`)))
    (if (<= _output_get 0.0)
      (`/Engine/EditorBlueprintResources/StandardMacros.DoOnce` false
        (:`Completed`
          (`GameplayStatics.SetGlobalTimeDilation` 1.0)
          (`self.HurtHighlight`)
          (`self.PlayAnimMontage` "/Game/Assets/Animations/Enemies/AM_GolemDeath.AM_GolemDeath")
          (`GameplayStatics.PlaySound2D` "/Game/SoundFX/MetaSounds/Implemented/MS_GolemDeathRubble.MS_GolemDeathRubble" 1.0 1.0 0.0 null null)
          (set `self.CanTakeDamage?` false)
          (`NiagaraFunctionLibrary.SpawnSystemAtLocation` "/Game/Assets/VFX/NS_CorpseExplosion.NS_CorpseExplosion" _returnvalue_2)
          (`KismetSystemLibrary.Delay` 0.5)
          (bind _returnvalue_4 (`GameplayStatics.GetActorOfClass` "/Game/AI/WaveLogic/BP_WaveManager.BP_WaveManager_C"))
          (`/Engine/EditorBlueprintResources/StandardMacros.IsValid` _returnvalue_4
            (:`Is Valid`
              (`/Game/AI/WaveLogic/BP_WaveManager.SubtractFromNeeded` _returnvalue_4))
            (:`Is Not Valid`
              _))
          (if (<= (`KismetMathLibrary.RandomInteger` 101) 90)
            (`|SpawnActorFromClass` "/Game/Assets/BluePrints/Pickups/BP_CollectableOrb.BP_CollectableOrb_C" (`KismetMathLibrary.MakeTransform` (`KismetMathLibrary.MakeVector` (.x (.location _returnvalue_3)) (.y (.location _returnvalue_3)) 65.0)) "Undefined" "OverrideRootScale" null null))
          (`self.K2_DestroyActor`))))))

(event `/Game/AI/EnemyFootsoldier/BPI_AICombat.AIMeleeHeavyAttack`
  ;[1 0.1195 0.1195] AI Melee
  (set `self.Is Immovable` true)
  (`self.PlayAnimMontage` "/Game/Assets/Animations/Enemies/AM_GolemHeavyAttack.AM_GolemHeavyAttack")
  (goto _label))

(event `AI Heavy Attack Trace`
  ;[1 0.1195 0.1195] AI Attack Sphere Trace Footsoldier
  (`self.GolemAttack` 25.0 1200.0 250.0))

(event `CheckAttack`
  ;[1 0.1195 0.1195] Checks attack
  (bind _outactors (`GameplayStatics.GetAllActorsOfClass` "BP_Golem_C"))
  (for _array_element _outactors
    (if (not (== _array_element self))
      (`BlackboardComponent.SetValueAsBool` (`AIBlueprintHelperLibrary.GetBlackboard` _array_element) "CanAttack?" true))))

(event `/Game/Assets/BluePrints/Interfaces/BPIDamageRecievers.Knockback`
  (params (KnockbackSource :type "Vector Structure") (KnockbackValue :type "Float (double-precision)") (`Launch Value` :type "Float (double-precision)"))
  ;[1 1 1] Damage and knockback
  (if (not (`self.Is Immovable`))
    (`|ExecutionSequence`
      (:`then_0`
        (set `self.Launch Value` `Launch Value`)
        (set `self.Knockback Value` KnockbackValue)
        (if (`self.FirstHit?`)
          (bind _result (`/Engine/EditorBlueprintResources/StandardMacros.IncrementInt` (`self.NumberOfHits`) :!label _label_2)
            (:`  `
              (set `self.NumberOfHits` _result)
              (set `self.FirstHit?` false)))
          (else
            (switch `int` (`self.NumberOfHits`)
              (:`0`
                (goto _label_2))
              (:`1`
                (`self.AddLaunch` 1.25))
              (:`2`
                (`self.AddLaunch` 1.5))
              (:`3`
                (`self.AddLaunch` 1.75))
              (:`4`
                (`self.AddLaunch` 2.5)
                (`self.AddKnockback` 30.0)))
            (bind _result_2 (`/Engine/EditorBlueprintResources/StandardMacros.IncrementInt` (`self.NumberOfHits`))
              (:`  `
                (set `self.NumberOfHits` _result_2)))))
        (`NavMovementComponent.StopActiveMovement` (`self.CharacterMovement`))
        (bind _applied_knockback (`self.Calculate KB Dir` KnockbackSource (`self.K2_GetActorLocation` self) (`self.Knockback Value`) (`self.Launch Value`)))
        (`self.LaunchCharacter` _applied_knockback true true)
        (`self.PlayAnimMontage` (`|GetArrayItem` (`self.HitAnims`) (`KismetMathLibrary.RandomIntegerInRange` 0 (- (`KismetArrayLibrary.Array_Length` (`self.HitAnims`)) 1))))
        (`/Engine/EditorBlueprintResources/StandardMacros.IsValid` (`self.Indicator`)
          (:`Is Valid`
            (`self.K2_DestroyActor` (`self.Indicator`)))
          (:`Is Not Valid`
            _))
        (if (>= (`self.NumberOfHits`) 5)
          (set `self.NumberOfHits` 0)))
      (:`then_1`
        (`KismetSystemLibrary.RetriggerableDelay` 1.5)
        (set `self.NumberOfHits` 0)))))

(event `BeforeDestroy`
  (bind _returnvalue (`AIBlueprintHelperLibrary.GetBlackboard` null))
  ;[1 0.1195 0.1195] Checks attack
  (if (== self (`BlackboardComponent.GetValueAsObject` _returnvalue "CurrentlyTango"))
    (`BlackboardComponent.SetValueAsObject` _returnvalue "CurrentlyTango" null)))

(event `self.ReceiveBeginPlay`
  ;[1 0.1195 0.1195] Comment
  (set `CharacterMovementComponent.MaxWalkSpeed` (`KismetMathLibrary.RandomFloatInRange` 200.0 500.0) (`self.CharacterMovement`))
  (bind _returnvalue (`GameplayStatics.GetActorOfClass` "/Game/AI/WaveLogic/BP_WaveManager.BP_WaveManager_C"))
  (`/Engine/EditorBlueprintResources/StandardMacros.IsValid` _returnvalue
    (:`Is Valid`
      (`/Game/AI/WaveLogic/BP_WaveManager.AddToNeeded` _returnvalue))
    (:`Is Not Valid`
      _))
  (`SceneComponent.K2_SetRelativeLocation` (`self.Mesh`) (0.0 0.0 -500.0) false true)
  (`KismetSystemLibrary.Delay` (`KismetMathLibrary.RandomFloatInRange` 0.5 1.0))
  (bind (_direction _risingeffect) (`Timeline|Rise`)
    (:`Update`
      (`SceneComponent.K2_SetRelativeLocation` (`self.Mesh`) (`KismetMathLibrary.MakeVector` 0.0 0.0 _risingeffect) false false))
    (:`Finished`
      (`AIController.RunBehaviorTree` (`AIBlueprintHelperLibrary.GetAIController` self) "/Game/AI/EnemyFootsoldier/BT_AIFS.BT_AIFS")
      (`BlackboardComponent.SetValueAsObject` (`AIBlueprintHelperLibrary.GetBlackboard` null) "TargetActor" (`GameplayStatics.GetPlayerCharacter` 0)))
    (:`Crack`
      (`NiagaraFunctionLibrary.SpawnSystemAtLocation` "/Game/Assets/VFX/MovementVFX/NS_Rupturetest.NS_Rupturetest" (- (`self.K2_GetActorLocation`) (0.0 0.0 90.0))))))

(fn `AddKnockback`
  (params (KnockbackBoost :type "Float (double-precision)"))
  (set `self.Knockback Value` (* KnockbackBoost (`self.Knockback Value`))))

(fn `AddLaunch`
  (params (LaunchBoost :type "Float (double-precision)"))
  (set `self.Launch Value` (* LaunchBoost (`self.Launch Value`))))

(fn `Calculate KB Dir`
  (params (`Knockback Source` :type "Vector Structure") (`My Position` :type "Vector Structure") (`Directional Strenght` :type "Float (double-precision)") (`Launch Strenght` :type "Float (double-precision)"))
  (returns (`Applied Knockback` :type "Vector Structure"))
  (locals (NewLocalVar :type "Float (double-precision)") (KnockbackDirection :type "Vector Structure"))
  (bind (_kbs_x _kbs_y _kbs_z) (`KismetMathLibrary.BreakVector` (`self.KBS`)))
  (bind (_mypos_x _mypos_y _mypos_z) (`KismetMathLibrary.BreakVector` (`self.MYPOS`)))
  (set `self.KBS` `Knockback Source`)
  (set `self.MYPOS` `My Position`)
  (bind _output_get (set `local.KnockbackDirection` (+ (`KismetMathLibrary.MakeVector` 0.0 0.0 `Launch Strenght`) (* `Directional Strenght` (`KismetMathLibrary.Normal` (- (- (`self.MYPOS`) (`KismetMathLibrary.MakeVector` 0.0 0.0 _mypos_z)) (- (`self.KBS`) (`KismetMathLibrary.MakeVector` 0.0 0.0 _kbs_z))))))))
  (return _output_get))

(fn `GolemAttack`
  (params (`Damage Taken` :type "Float (double-precision)") (KnockbackValue :type "Float (double-precision)") (`Launch Value` :type "Float (double-precision)"))
  (bind _returnvalue (`SceneComponent.K2_GetComponentLocation` (`self.SphereTraceAttack`)))
  (bind _outhits (`KismetSystemLibrary.CapsuleTraceMultiForObjects` _returnvalue _returnvalue 150.0 100.0 (`self.object types`)))
  (for _array_element _outhits
    (bind _asbp_main_character (cast `/Game/Assets/BluePrints/MainCharacter/BP_MainCharacter` (`.HitActor` (`GameplayStatics.BreakHitResult` _array_element))))
    (if (`self.Can damage?`)
      (message `/Game/Assets/BluePrints/Interfaces/BPIDamageRecievers.TakeDamage` _asbp_main_character `Damage Taken` 0.0)
      (set `self.Can damage?` false)
      (message `/Game/Assets/BluePrints/Interfaces/BPIDamageRecievers.Knockback` _asbp_main_character (`self.K2_GetActorLocation`) KnockbackValue `Launch Value`))))

(fn `UserConstructionScript`)