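; A one-sided door that lets the main character through, then restores its collision and starts the boss encounter.
; An Entry overlap turns off the door mesh's collision; an Exit overlap sets it to query-only, calls StartAllLogic on BP_BossMan and fades in boss music.
; Each trigger's DoOnce precedes the character cast, so the first overlap by any actor uses it up.
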(event `self.Entry.OnComponentBeginOverlap`
  (params (OverlappedComponent :type "PrimitiveComponent Object Reference") (OtherActor :type "Actor Object Reference") (OtherComp :type "PrimitiveComponent Object Reference") (OtherBodyIndex :type Integer) (bFromSweep :type Boolean) (SweepResult :type "HitResult Structure (by ref)"))
  (`/Engine/EditorBlueprintResources/StandardMacros.DoOnce` false
    (:`Completed`
      (cast `/Game/Assets/BluePrints/MainCharacter/BP_MainCharacter` OtherActor)
      (`PrimitiveComponent.SetCollisionEnabled` (`StaticMeshActor.StaticMeshComponent` (`self.ActualMesh`)) "NoCollision"))))

(event `self.Exit.OnComponentBeginOverlap`
  (params (OverlappedComponent :type "PrimitiveComponent Object Reference") (OtherActor :type "Actor Object Reference") (OtherComp :type "PrimitiveComponent Object Reference") (OtherBodyIndex :type Integer) (bFromSweep :type Boolean) (SweepResult :type "HitResult Structure (by ref)"))
  (`/Engine/EditorBlueprintResources/StandardMacros.DoOnce` false
    (:`Completed`
      (cast `/Game/Assets/BluePrints/MainCharacter/BP_MainCharacter` OtherActor)
      (`PrimitiveComponent.SetCollisionEnabled` (`StaticMeshActor.StaticMeshComponent` (`self.ActualMesh`)) "QueryOnly")
      (bind _returnvalue (`GameplayStatics.GetActorOfClass` "/Game/AI/Bos/BP_BossMan.BP_BossMan_C"))
      (`/Game/AI/Bos/BP_BossMan.StartAllLogic` _returnvalue)
      (`AudioComponent.FadeIn` (`AmbientSound.AudioComponent` (`self.BossMusic`)) 1.0 1.0 0.0 "Linear"))))

(fn `UserConstructionScript`)