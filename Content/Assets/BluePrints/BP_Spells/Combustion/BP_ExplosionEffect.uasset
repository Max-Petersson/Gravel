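; BP_ExplosionEffect is the short-lived blast actor of the Combustion spell, hitting damageable actors around where it spawns.
; On BeginPlay a sphere trace finds BPIDamageRecievers and messages them through that interface.
; The main character gets only a knockback launch, while others take knockback, health and poise damage once each, tracked in HitActors.
; It destroys itself after a short delay, and its spell functions are empty stubs.
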(event `self.ReceiveBeginPlay`
  (bind _returnvalue (`self.K2_GetActorLocation`))
  (bind _outhits (`KismetSystemLibrary.SphereTraceMultiForObjects` _returnvalue _returnvalue 125.0 (`self.Affected`)))
  (for _array_element _outhits
    (bind _asbpidamage_recievers (cast `/Game/Assets/BluePrints/Interfaces/BPIDamageRecievers` (`.HitActor` (`GameplayStatics.BreakHitResult` _array_element))))
    (if (not (`KismetArrayLibrary.Array_Contains` (`self.Hit Actors`) _asbpidamage_recievers))
      (bind _returnvalue_2 (`KismetSystemLibrary.Conv_InterfaceToObject` _asbpidamage_recievers))
      (cast `/Game/Assets/BluePrints/MainCharacter/BP_MainCharacter` _returnvalue_2
        (:`then`
          (message `/Game/Assets/BluePrints/Interfaces/BPIDamageRecievers.Knockback` _returnvalue_2 (`self.K2_GetActorLocation`) 2.0 (`self.Player Launch`)))
        (:`CastFailed`
          (message `/Game/Assets/BluePrints/Interfaces/BPIDamageRecievers.Knockback` _returnvalue_2 (`self.K2_GetActorLocation`) 1.0 500.0)
          ;[1 1 1] Damage could scale with a parameter from CastSpell
          (message `/Game/Assets/BluePrints/Interfaces/BPIDamageRecievers.TakeDamage` _returnvalue_2 75.0 30.0)
          (`KismetArrayLibrary.Array_Add` (`self.Hit Actors`) _asbpidamage_recievers)))))
  (`KismetSystemLibrary.Delay` 1.2)
  (`self.K2_DestroyActor`)
  (`KismetArrayLibrary.Array_Clear` (`self.Hit Actors`)))

(fn `Ask for spell`
  (returns (NewParam :type Boolean))
  (return false))

(fn `execute spell`)

(fn `UserConstructionScript`)