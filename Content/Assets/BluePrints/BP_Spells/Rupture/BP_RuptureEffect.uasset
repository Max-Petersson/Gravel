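; BP_RuptureEffect is the moving effect actor for the Rupture spell, launching targets it passes through.
; Collider overlaps send a knockback message with launch force but zero knockback to actors implementing BPIDamageRecievers, using a Hits list so each is affected only once.
; After a short delay from BeginPlay it stops its projectile movement and removes the collider, then lingers briefly before destroying itself.
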(event `self.ReceiveBeginPlay`
  (`KismetSystemLibrary.Delay` 1.0)
  (`MovementComponent.StopMovementImmediately` (`self.ProjectileMovement`))
  (`ActorComponent.K2_DestroyComponent` (`self.Collider`))
  (`KismetSystemLibrary.Delay` 2.0)
  (`self.K2_DestroyActor`))

(event `self.Collider.OnComponentBeginOverlap`
  (params (OverlappedComponent :type "PrimitiveComponent Object Reference") (OtherActor :type "Actor Object Reference") (OtherComp :type "PrimitiveComponent Object Reference") (OtherBodyIndex :type Integer) (bFromSweep :type Boolean) (SweepResult :type "HitResult Structure (by ref)"))
  (bind _asbpidamage_recievers (cast `/Game/Assets/BluePrints/Interfaces/BPIDamageRecievers` OtherActor))
  (if (not (`KismetArrayLibrary.Array_Contains` (`self.Hits`) _asbpidamage_recievers))
    (`KismetArrayLibrary.Array_Add` (`self.Hits`) _asbpidamage_recievers)
    (message `/Game/Assets/BluePrints/Interfaces/BPIDamageRecievers.Knockback` (`KismetSystemLibrary.Conv_InterfaceToObject` _asbpidamage_recievers) (`self.K2_GetActorLocation`) 0.0 500.0)))

(fn `UserConstructionScript`)