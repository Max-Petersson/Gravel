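; BPC_Combust is a spell that creates an explosion effect at an aimed location.
; On BeginPlay it sets itself as the EquippedSpell on the player's BP_MainCharacter.
; It spawns a BP_ExplodeVisualisation as an aiming preview and moves it to each aimed location it receives.
; CastSpell spawns BP_ExplosionEffect there with the given rotation and owner, then destroys the preview.
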(event `/Game/Assets/BluePrints/BP_Spells/BaseClass/BPI_SpellEffects.CastSpell`
  (params (AimedLocation :type "Vector Structure") (SpawnRotation :type "Rotator Structure") (Owner :type "Actor Object Reference") (SocketLocation :type "Vector Structure") (BaseDamage :type "Float (double-precision)"))
  (`|SpawnActorFromClass` "/Game/Assets/BluePrints/BP_Spells/Combustion/BP_ExplosionEffect.BP_ExplosionEffect_C" (`KismetMathLibrary.MakeTransform` AimedLocation SpawnRotation) "Undefined" "OverrideRootScale" Owner null)
  (`self.K2_DestroyActor` (`self.Visu`)))

(event `self.ReceiveBeginPlay`
  (bind _asbp_main_character (cast `/Game/Assets/BluePrints/MainCharacter/BP_MainCharacter` (`GameplayStatics.GetPlayerCharacter` 0)))
  (set `/Game/Assets/BluePrints/MainCharacter/BP_MainCharacter.Equipped Spell` self _asbp_main_character))

(event `/Game/Assets/BluePrints/BP_Spells/BaseClass/BPI_SpellEffects.Move Visualisation`
  (params (AimedLocation :type "Vector Structure") (SpawnRotation :type "Rotator Structure") (Owner :type "Actor Object Reference") (SocketLocation :type "Vector Structure") (BaseDamage :type "Float (double-precision)"))
  (`self.K2_SetActorLocation` (`self.Visu`) AimedLocation false false))

(event `/Game/Assets/BluePrints/BP_Spells/BaseClass/BPI_SpellEffects.SpawnVisualisation`
  (params (AimedLocation :type "Vector Structure") (SpawnRotation :type "Rotator Structure") (Owner :type "Actor Object Reference") (SocketLocation :type "Vector Structure") (BaseDamage :type "Float (double-precision)"))
  (bind _returnvalue (`|SpawnActorFromClass` "/Game/Assets/BluePrints/BP_Spells/Combustion/BP_ExplodeVisualisation.BP_ExplodeVisualisation_C" (`KismetMathLibrary.MakeTransform` AimedLocation) "Undefined" "OverrideRootScale" null null))
  (set `self.Visu` _returnvalue))

(fn `UserConstructionScript`
  (`parent.UserConstructionScript`))