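; BP_CheckpointManager restores the player to a saved spawn point when play begins, if a save game exists.
; Its construction script copies the save slot name from the first BP_SpawnPoint actor found.
; BeginPlay loads BP_SaveGame from that slot, waits a tick, then moves the player character to the stored transform.
; It disables movement behind a loading screen widget for a fixed delay, then restores walking and removes the widget.
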(event `self.ReceiveBeginPlay`
  (bind _returnvalue (`GameplayStatics.GetPlayerCharacter` 0))
  (bind _charactermovement (`Character.CharacterMovement` _returnvalue))
  (bind _returnvalue_2 (`GameplayStatics.DoesSaveGameExist` (`self.Slot Name`)))
  (if _returnvalue_2
    (bind _returnvalue_3 (`GameplayStatics.LoadGameFromSlot` (`self.Slot Name`)))
    (bind _asbp_save_game (cast `/Game/Assets/BluePrints/Respawn/BP_SaveGame` _returnvalue_3))
    (`KismetSystemLibrary.DelayUntilNextTick`)
    (`self.K2_SetActorTransform` _returnvalue (`/Game/Assets/BluePrints/Respawn/BP_SaveGame.Spawn Point` _asbp_save_game) false false)
    (`CharacterMovementComponent.SetMovementMode` _charactermovement "MOVE_None" 0)
    (bind _returnvalue_4 (`|CreateWidget` "/Game/Assets/WBP_LoadingScreen.WBP_LoadingScreen_C" (`GameplayStatics.GetPlayerController` 0)))
    (`UserWidget.AddToViewport` _returnvalue_4 0)
    (`KismetSystemLibrary.Delay` 3.0)
    (`CharacterMovementComponent.SetMovementMode` _charactermovement "MOVE_Walking" 0)
    (`Widget.RemoveFromParent` _returnvalue_4)))

(fn `UserConstructionScript`
  (bind _returnvalue (`GameplayStatics.GetActorOfClass` "/Game/Assets/BluePrints/Respawn/BP_SpawnPoint.BP_SpawnPoint_C"))
  (`/Engine/EditorBlueprintResources/StandardMacros.IsValid` _returnvalue
    (:`Is Valid`
      (set `self.Slot Name` (`/Game/Assets/BluePrints/Respawn/BP_SpawnPoint.Slot Name` _returnvalue)))))