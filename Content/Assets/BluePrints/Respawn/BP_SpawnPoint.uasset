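; BP_SpawnPoint is a checkpoint actor that saves the player's respawn location when BP_MainCharacter enters its TriggerCheckPoint volume.
; The overlap fires once through a DoOnce, then loads the existing BP_SaveGame from the slot or creates a new one.
; It writes the SpawnPoint component's world transform, sets ShouldBossStart when IsBoss is on, and saves back to the slot.
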(event `self.TriggerCheckPoint.OnComponentBeginOverlap`
  (params (OverlappedComponent :type "PrimitiveComponent Object Reference") (OtherActor :type "Actor Object Reference") (OtherComp :type "PrimitiveComponent Object Reference") (OtherBodyIndex :type Integer) (bFromSweep :type Boolean) (SweepResult :type "HitResult Structure (by ref)"))
  (cast `/Game/Assets/BluePrints/MainCharacter/BP_MainCharacter` OtherActor)
  (`/Engine/EditorBlueprintResources/StandardMacros.DoOnce` false
    (:`Completed`
      (bind _returnvalue (`GameplayStatics.DoesSaveGameExist` (`self.Slot Name`)))
      (if _returnvalue
        (bind _returnvalue_2 (`GameplayStatics.LoadGameFromSlot` (`self.Slot Name`)))
        (bind _asbp_save_game (cast `/Game/Assets/BluePrints/Respawn/BP_SaveGame` _returnvalue_2))
        (set `/Game/Assets/BluePrints/Respawn/BP_SaveGame.Spawn Point` (`SceneComponent.K2_GetComponentToWorld` (`self.SpawnPoint`)) _asbp_save_game)
        (if (`self.IsBoss?`)
          (set `/Game/Assets/BluePrints/Respawn/BP_SaveGame.ShouldBossStart+` true _asbp_save_game))
        (`GameplayStatics.SaveGameToSlot` _asbp_save_game (`self.Slot Name`))
        (else
          (bind _returnvalue_3 (`GameplayStatics.CreateSaveGameObject` "/Game/Assets/BluePrints/Respawn/BP_SaveGame.BP_SaveGame_C"))
          (set `/Game/Assets/BluePrints/Respawn/BP_SaveGame.Spawn Point` (`SceneComponent.K2_GetComponentToWorld` (`self.SpawnPoint`)) _returnvalue_3)
          (if (`self.IsBoss?`)
            (set `/Game/Assets/BluePrints/Respawn/BP_SaveGame.ShouldBossStart+` true _returnvalue_3))
          (`GameplayStatics.SaveGameToSlot` _returnvalue_3 (`self.Slot Name`)))))))

(fn `UserConstructionScript`)