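; BP_Dummy is a Character that acts as a damageable target which can be knocked back.
; TakeDamage prints a debug string, subtracts the damage from Health and destroys the actor at zero or below.
; Knockback launches the character away from the source point, scaling the unnormalized offset by the knockback value, so launch strength grows with distance.
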(event `/Game/Assets/BluePrints/Interfaces/BPIDamageRecievers.TakeDamage`
  (params (`Damage Taken` :type "Float (double-precision)"))
  (`KismetSystemLibrary.PrintString` "Hello")
  (set `self.Health` (- (`self.Health`) `Damage Taken`))
  (if (<= (`self.Health`) 0.0)
    (`self.K2_DestroyActor`)))

(event `/Game/Assets/BluePrints/Interfaces/BPIDamageRecievers.Knockback`
  (params (KnockbackSource :type "Vector Structure") (KnockbackValue :type "Float (double-precision)"))
  (`self.LaunchCharacter` (* KnockbackValue (- (`self.K2_GetActorLocation`) KnockbackSource))))

(fn `UserConstructionScript`)