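; Hammer melee component for BP_ThirdPersonCharacter that runs a three-montage attack combo and applies hit damage.
; Input during an attack is buffered in SaveAttack, and HammerAttackCombo either plays the next montage by AttackIndex or resets the combo.
; A looping timer sphere-traces between the hammer's top and bottom points, with a shared DoOnce cooldown limiting damage.
; A separate one-shot sphere trace handles thrusts; both damage only BPI_Test_E implementers.
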(event `self.ReceiveBeginPlay`
  (bind _asbp_third_person_character (cast `/Game/ThirdPerson/Blueprints/BP_ThirdPersonCharacter` (`self.GetOwner`)))
  (set `self.Character BP` _asbp_third_person_character)
  (set `self.carachterMesh` (`Character.Mesh` _asbp_third_person_character)))

(event `EnhancedInput|/Game/Assets/Input/Actions/IA_Attack_M1`
  (params (ActionValue :type Boolean) (ElapsedSeconds :type "Float (double-precision)") (TriggeredSeconds :type "Float (double-precision)") (InputAction :type "InputAction Object Reference" :default "/Game/Assets/Input/Actions/IA_Attack_M1.IA_Attack_M1"))
  ;[0.1594 1 0.332] Combo System
  ;;[1 1 1] Attack Input
  (:`Started`
    (if (`self.canAttack?`)
      (`self.Hammer Attack`))))

(event `Attack 1`
  ;[0.1594 1 0.332] Combo System
  ;;[1 1 1] Attack 1
  (`/Engine/EditorBlueprintResources/StandardMacros.DoOnce` false :!label _label
    (:`Completed`
      (`KismetSystemLibrary.Delay` 0.1)
      (`|PlayMontage` (`self.carachterMesh`) "/Game/Characters/Player_Character/Animations/HammerAttacks/Attack1_Montage.Attack1_Montage"
        (:`then`
          (set `self.attackIndex` 1)
          (goto _label :!via `Reset`))))))

(event `Hammer Attack`
  ;[0.1594 1 0.332] Combo System
  ;;[1 1 1] Hammer Attack
  (if (`self.isAttacking?`)
    (set `self.saveAttack?` true)
    (else
      (set `self.isAttacking?` true)
      (switch `int` (`self.attackIndex`) :!label _label_2
        (:`0`
          (`self.Attack 1`))
        (:`1`
          (`self.Attack 2`))
        (:`2`
          (`self.Attack 3`))))))

(event `Attack 2`
  ;[0.1594 1 0.332] Combo System
  ;;[1 1 1] Attack 2
  (`/Engine/EditorBlueprintResources/StandardMacros.DoOnce` false :!label _label_3
    (:`Completed`
      (`KismetSystemLibrary.Delay` 0.1)
      (`|PlayMontage` (`self.carachterMesh`) "/Game/Characters/Player_Character/Animations/HammerAttacks/Attack2_Montage.Attack2_Montage"
        (:`then`
          (set `self.attackIndex` 2)
          (goto _label_3 :!via `Reset`))))))

(event `Hammer Attack Combo`
  ;[0.1594 1 0.332] Combo System
  ;;[1 1 1] Combo Continue
  (if (`self.saveAttack?`)
    (set `self.saveAttack?` false)
    (goto _label_2)
    (else
      (`self.Stop Combo`))))

(event `Attack 3`
  ;[0.1594 1 0.332] Combo System
  ;;[1 1 1] Attack 3
  (`/Engine/EditorBlueprintResources/StandardMacros.DoOnce` false :!label _label_4
    (:`Completed`
      (`KismetSystemLibrary.Delay` 0.1)
      (`|PlayMontage` (`self.carachterMesh`) "/Game/Characters/Player_Character/Animations/HammerAttacks/Attack3_Montage.Attack3_Montage"
        (:`then`
          (set `self.attackIndex` 3)
          (goto _label_4 :!via `Reset`))))))

(event `Stop Combo`
  ;[0.1594 1 0.332] Combo System
  ;;[1 1 1] Stop Combo/Attack
  (set `self.isAttacking?` false)
  (set `self.attackIndex` 0))

(event `Start Hammer Trace`
  ;[0.159 1 0.3325] Hammer Trace
  (bind _returnvalue (`KismetSystemLibrary.K2_SetTimerDelegate` (delegate `Hammer Trace Loop`) 0.001 true))
  (set `self.HammerTraceLoop` _returnvalue))

(event `Sphere Trace`
  (bind _character_bp (`self.Character BP`))
  (bind _returnvalue (`SceneComponent.K2_GetComponentLocation` (`/Game/ThirdPerson/Blueprints/BP_ThirdPersonCharacter.SphereTrace` _character_bp)))
  ;[0.1594 1 0.332] Sphere Trace (For Hammer Thrust)
  (bind (_outhits _returnvalue_2) (`KismetSystemLibrary.SphereTraceMultiForObjects` _returnvalue _returnvalue 60.0 (`self.Object Types`) false (`|MakeArray` _character_bp :!type "Actor Object Reference") "ForDuration"))
  (for _array_element _outhits
    (if _returnvalue_2
      (bind (_bblockinghit _binitialoverlap _time _distance _location _impactpoint _normal _impactnormal _physmat _hitactor) (`GameplayStatics.BreakHitResult` _array_element))
      (if (`KismetSystemLibrary.DoesImplementInterface` _hitactor "/Game/Assets/BluePrints/Erik/BPI_Test_E.BPI_Test_E_C")
        (`GameplayStatics.ApplyDamage` _hitactor 10.0)))))

(event `Hammer Trace Loop`
  (bind _character_bp (`self.Character BP`))
  ;[0.159 1 0.3325] Hammer Trace
  (bind (_outhits _returnvalue) (`KismetSystemLibrary.SphereTraceMultiForObjects` (`SceneComponent.K2_GetComponentLocation` (`/Game/ThirdPerson/Blueprints/BP_ThirdPersonCharacter.HammerTopPoint` _character_bp)) (`SceneComponent.K2_GetComponentLocation` (`/Game/ThirdPerson/Blueprints/BP_ThirdPersonCharacter.HammerBottomPoint` (`self.Character BP`))) 25.0 (`self.Object Types`) false (`|MakeArray` _character_bp :!type "Actor Object Reference") "ForDuration"))
  (for _array_element _outhits
    (if _returnvalue
      (bind (_bblockinghit _binitialoverlap _time _distance _location _impactpoint _normal _impactnormal _physmat _hitactor) (`GameplayStatics.BreakHitResult` _array_element))
      (if (`KismetSystemLibrary.DoesImplementInterface` _hitactor "/Game/Assets/BluePrints/Erik/BPI_Test_E.BPI_Test_E_C")
        (`/Engine/EditorBlueprintResources/StandardMacros.DoOnce` false :!label _label_5
          (:`Completed`
            (`GameplayStatics.ApplyDamage` _hitactor 10.0)
            (`KismetSystemLibrary.Delay` 0.5)
            (goto _label_5 :!via `Reset`)))))))

(event `Stop Hammer Trace`
  ;[0.159 1 0.3325] Hammer Trace
  (`KismetSystemLibrary.K2_ClearAndInvalidateTimerHandle` (`self.HammerTraceLoop`)))