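; Health component for the main character that tracks current and max health, updates the HUD health bar and handles death.
; Heal and damage functions clamp health, then trigger healing particles or a damage vignette respectively.
; Over-time events loop on a Delay, applying equal slices at a Smoothness interval through those same functions.
; Reaching zero health calls Mortis, which blocks player input and shows the death canvas.
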(event `self.ReceiveBeginPlay`
  (bind _asbp_main_character (cast `/Game/Assets/BluePrints/MainCharacter/BP_MainCharacter` (`self.GetOwner`)))
  (bind _output_get (set `self.PlayerCharacter_REF` _asbp_main_character))
  (`KismetSystemLibrary.DelayUntilNextTick`)
  (set `self.HUD_PlayerRef` (`/Game/Assets/BluePrints/MainCharacter/BP_MainCharacter.HUD Ref` _output_get)))

(event `IncreaseHealthOverTime`
  (params (HealAmount :type "Float (double-precision)") (HealDuration :type "Float (double-precision)"))
  (bind _smoothness (`self.Smoothness`))
  ;[1 1 1] Increases a set amount of curse evenly over a certain amount of time
  (set `self.TimeLeft` HealDuration)
  (bind _output_get (set `self.Heal Duration` HealDuration))
  (`self.IncreaseHealth` (* (/ HealAmount _output_get) (`self.Smoothness`)) :!label _label)
  (`KismetSystemLibrary.Delay` _smoothness)
  (bind _output_get_2 (set `self.TimeLeft` (- (`self.TimeLeft`) _smoothness)))
  (if (not (<= _output_get_2 0.0))
    (goto _label)))

(event `DecreaseHealthOverTime`
  (params (DamageAmount :type "Float (double-precision)") (DamageDuration :type "Float (double-precision)"))
  (bind _smoothness (`self.Smoothness`))
  ;[1 1 1] Decreases a set amount of curse evenly over a certain amount of time
  (set `self.TimeLeftToHeal` DamageDuration)
  (bind _output_get (set `self.Damage Duration ` DamageDuration))
  (`self.DecreaseHealth` (* (/ DamageAmount _output_get) (`self.Smoothness`)) :!label _label_2)
  (`KismetSystemLibrary.Delay` _smoothness)
  (bind _output_get_2 (set `self.TimeLeftToHeal` (- (`self.TimeLeftToHeal`) _smoothness)))
  (if (not (<= _output_get_2 0.0))
    (goto _label_2)))

(event `Mortis`
  (`KismetSystemLibrary.PrintString` "MORTIS")
  (set `/Game/Assets/BluePrints/MainCharacter/BP_MainCharacter.BlockInput?` true (`self.PlayerCharacter_REF`))
  (`Widget.SetVisibility` (`/Game/UI/WBP_HUD.Canvas_Death` (`self.HUD_PlayerRef`)) "Visible"))

(fn `DecreaseHealth`
  (params (`Curse Amount` :type "Float (double-precision)"))
  (bind _hud_playerref (`self.HUD_PlayerRef`))
  (bind _currenthealth (`self.CurrentHealth`))
  (set `self.CurrentHealth` (`KismetMathLibrary.FClamp` (- (`self.CurrentHealth`) `Curse Amount`) 0.0 (`self.MaxHealth`)))
  (`ProgressBar.SetPercent` (`/Game/UI/WBP_HUD.HealthBar` _hud_playerref) (/ _currenthealth (`self.MaxHealth`)))
  (`/Game/UI/WBP_HUD.EnableDamageVingette` _hud_playerref)
  (if (== _currenthealth 0.0)
    (`self.Mortis`)))

(fn `IncreaseHealth`
  (params (`Curse Amount` :type "Float (double-precision)"))
  (returns (`PlayerDead?` :type Boolean))
  (bind _currenthealth (`self.CurrentHealth`))
  (bind _maxhealth (`self.MaxHealth`))
  (set `self.CurrentHealth` (`KismetMathLibrary.FClamp` (+ `Curse Amount` (`self.CurrentHealth`)) 0.0 (`self.MaxHealth`)))
  (`ProgressBar.SetPercent` (`/Game/UI/WBP_HUD.HealthBar` (`self.HUD_PlayerRef`)) (/ _currenthealth _maxhealth))
  (`NiagaraFunctionLibrary.SpawnSystemAtLocation` "/Game/Assets/VFX/NS_HealingParticles.NS_HealingParticles" (`SceneComponent.K2_GetComponentLocation` (`Actor.RootComponent` (`self.PlayerCharacter_REF`))))
  (if (>= _currenthealth _maxhealth)
    (return true)
    (else
      (return false))))

(fn `IncreaseMaxHealth`
  (params (`Curse Amount` :type "Float (double-precision)"))
  (set `self.MaxHealth` (+ `Curse Amount` (`self.MaxHealth`))))