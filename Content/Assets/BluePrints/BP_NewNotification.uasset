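; Trigger actor that shows a notification widget, through BPI_Notifications, the first time BP_MainCharacter enters its box.
; It either shows a popup or pauses the game with a full notification registered with BP_NotificationManager.
; EndPauseScreen unpauses and swaps the notification for the popup.
; The popup is removed via the EndNotify box when box-bound, or by a one-second poll once all KillsNeeded actors are invalid when kill-dependent.
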(event `Check for kills`
  (`KismetSystemLibrary.Delay` 1.0 :!label _label)
  (set `self.KillListEmpty?` true)
  (for _array_element (`self.KillsNeeded`)
    (`/Engine/EditorBlueprintResources/StandardMacros.IsValid` _array_element
      (:`Is Valid`
        (set `self.KillListEmpty?` false)
        (`|ExecutionSequence`
          (:`then_0`
            (break))
          (:`then_1`
            (goto _label))))))
  (if (`self.KillListEmpty?`)
    (`/Game/Assets/UI/HUD_Notifications/BPI_Notifications.RemovePopUp` (`self.ActualWidget`))))

(event `self.ReceiveBeginPlay`
  (if (`self.IsKillDependant?`)
    (`self.Check for kills`)))

(event `self.Box.OnComponentBeginOverlap`
  (params (OverlappedComponent :type "PrimitiveComponent Object Reference") (OtherActor :type "Actor Object Reference") (OtherComp :type "PrimitiveComponent Object Reference") (OtherBodyIndex :type Integer) (bFromSweep :type Boolean) (SweepResult :type "HitResult Structure (by ref)"))
  (cast `/Game/Assets/BluePrints/MainCharacter/BP_MainCharacter` OtherActor)
  (`/Engine/EditorBlueprintResources/StandardMacros.DoOnce` false
    (:`Completed`
      (bind _returnvalue (`|CreateWidget` (`self.NotificationWidget`) (`GameplayStatics.GetPlayerController` 0)))
      (set `self.Widgett` _returnvalue)
      (bind _asbpi_notifications (cast `/Game/Assets/UI/HUD_Notifications/BPI_Notifications` _returnvalue))
      (set `self.ActualWidget` _asbpi_notifications)
      (if (`self.ShouldPauseGame?`)
        (set `PlayerController.bShowMouseCursor` true (`GameplayStatics.GetPlayerController` 0))
        (`GameplayStatics.SetGamePaused` true)
        (bind _returnvalue_2 (`GameplayStatics.GetActorOfClass` "/Game/Assets/BluePrints/BP_NotificationManager.BP_NotificationManager_C"))
        (`/Engine/EditorBlueprintResources/StandardMacros.IsValid` _returnvalue_2
          (:`Is Valid`
            (set `/Game/Assets/BluePrints/BP_NotificationManager.CurrentNotification` self _returnvalue_2)
            (`UserWidget.AddToViewport` (`self.Widgett`) 0)
            (`/Game/Assets/UI/HUD_Notifications/BPI_Notifications.AddNotification` (`self.ActualWidget`))))
        (else
          (`self.Notification PopUp`))))))

(event `EndPauseScreen`
  (bind _actualwidget (`self.ActualWidget`))
  (set `PlayerController.bShowMouseCursor` false (`GameplayStatics.GetPlayerController` 0))
  (`GameplayStatics.SetGamePaused` false)
  (`/Engine/EditorBlueprintResources/StandardMacros.IsValid` (`KismetSystemLibrary.Conv_InterfaceToObject` _actualwidget)
    (:`Is Valid`
      (`/Game/Assets/UI/HUD_Notifications/BPI_Notifications.RemoveNotification` _actualwidget)
      (`KismetSystemLibrary.Delay` 0.5)
      (`self.Notification PopUp`))))

(event `self.EndNotify.OnComponentBeginOverlap`
  (params (OverlappedComponent :type "PrimitiveComponent Object Reference") (OtherActor :type "Actor Object Reference") (OtherComp :type "PrimitiveComponent Object Reference") (OtherBodyIndex :type Integer) (bFromSweep :type Boolean) (SweepResult :type "HitResult Structure (by ref)"))
  (if (`self.IsBoxBound?`)
    (cast `/Game/Assets/BluePrints/MainCharacter/BP_MainCharacter` OtherActor)
    (`KismetSystemLibrary.RetriggerableDelay` 0.5)
    (`/Engine/EditorBlueprintResources/StandardMacros.IsValid` (`self.Widgett`)
      (:`Is Valid`
        (`/Game/Assets/UI/HUD_Notifications/BPI_Notifications.RemovePopUp` (`self.ActualWidget`))))))

(fn `Notification PopUp`
  (`/Game/Assets/UI/HUD_Notifications/BPI_Notifications.AddPopUp` (`self.ActualWidget`)))

(fn `UserConstructionScript`)