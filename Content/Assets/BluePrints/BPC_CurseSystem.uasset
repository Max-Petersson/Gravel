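; Actor component that tracks a curse meter for BP_EmilCharacter and shows it on the HUD's CurseBar.
; IncreaseCurse and DecreaseCurse clamp the value between zero and MaxCurse, then update the bar percentage.
; IncreaseCurseOverTime spreads an amount over a duration through a Delay loop stepped by Smoothness.
; The over-max check follows the clamp, so IncreaseCurse returns false whenever MaxCurse is non-negative; debug prints remain.
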(event `self.ReceiveBeginPlay`
  (bind _asbp_emil_character (cast `/Game/Assets/BluePrints/BP_EmilCharacter` (`self.GetOwner`)))
  (set `self.PlayerCharacter_REF` _asbp_emil_character))

(event `IncreaseCurseOverTime`
  (params (CurseAmount :type "Float (double-precision)") (CurseDuration :type "Float (double-precision)"))
  (bind _smoothness (`self.Smoothness`))
  (set `self.TimeLeft` CurseDuration)
  (bind _output_get (set `self.Curse Duration` CurseDuration))
  (`self.IncreaseCurse` (* (/ CurseAmount _output_get) (`self.Smoothness`)) :!label _label)
  (`KismetSystemLibrary.Delay` _smoothness)
  (bind _output_get_2 (set `self.TimeLeft` (- (`self.TimeLeft`) _smoothness)))
  (if (not (<= _output_get_2 0.0))
    (`KismetSystemLibrary.PrintString` (`KismetStringLibrary.Conv_DoubleToString` _output_get_2))
    (goto _label)))

(fn `DecreaseCurse`
  (params (`Curse Amount` :type "Float (double-precision)"))
  (bind _currentcurse (`self.CurrentCurse`))
  (bind _maxcurse (`self.MaxCurse`))
  (set `self.CurrentCurse` (`KismetMathLibrary.FClamp` (- (`self.CurrentCurse`) `Curse Amount`) 0.0 (`self.MaxCurse`)))
  (`ProgressBar.SetPercent` (`/Game/UI/WBP_HUD.CurseBar` (`/Game/Assets/BluePrints/BP_EmilCharacter.HUD_REF` (`self.PlayerCharacter_REF`))) (/ _currentcurse _maxcurse))
  (if (> _currentcurse _maxcurse)
    _))

(fn `IncreaseCurse`
  (params (`Curse Amount` :type "Float (double-precision)"))
  (returns (`PlayerDead?` :type Boolean))
  (bind _currentcurse (`self.CurrentCurse`))
  (bind _maxcurse (`self.MaxCurse`))
  (bind _returnvalue (/ _currentcurse _maxcurse))
  (set `self.CurrentCurse` (`KismetMathLibrary.FClamp` (+ `Curse Amount` (`self.CurrentCurse`)) 0.0 (`self.MaxCurse`)))
  (`ProgressBar.SetPercent` (`/Game/UI/WBP_HUD.CurseBar` (`/Game/Assets/BluePrints/BP_EmilCharacter.HUD_REF` (`self.PlayerCharacter_REF`))) _returnvalue)
  (`KismetSystemLibrary.PrintString` (`KismetStringLibrary.Conv_DoubleToString` _returnvalue))
  (if (> _currentcurse _maxcurse)
    (return true)
    (else
      (return false))))