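; Main character component that runs hammer melee combat: light combo attacks, a heavy spin, a ground slam and a rupture effect.
; Attacks play montages and set damage or hitbox values, with a short timing window selecting the second light swing.
; Separate events run two box traces or a slam sphere trace, sending de-duplicated damage and knockback messages.
; Box hits add hammer charge by target type; the hammer-sweep trace is disconnected.
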(event `self.ReceiveBeginPlay`
  (bind _asbp_main_character (cast `/Game/Assets/BluePrints/MainCharacter/BP_MainCharacter` (`self.GetOwner`)))
  (set `self.Character_REF` _asbp_main_character)
  (set `self.carachterMesh` (`Character.Mesh` _asbp_main_character)))

(event `Light Attack`
  ;[0.1594 1 0.332] Combo System
  ;;[1 1 1] Attack Input
  (if (`self.canAttack?`)
    (if (`self.isSlamming?`)
      _
      (elif (`self.secondAttack?`)
        (`self.LightHammerAttack2`)
        (else
          (`self.Light Hammer Attack`))))))

(event `Attack 1`
  ;[0.1594 1 0.332] Combo System
  ;;[1 1 1] Anim_Light Attack
  (`/Engine/EditorBlueprintResources/StandardMacros.DoOnce` false :!label _label
    (:`Completed`
      (`self.SetHitboxVariables` (`KismetMathLibrary.MakeTransform` (250.0 0.0 0.0) (struct) (80.0 200.0 100.0)) (`KismetMathLibrary.MakeTransform` (100.0 0.0 0.0) (struct) (50.0 100.0 100.0)))
      (`|PlayMontage` (`self.carachterMesh`) "/Game/Assets/Animations/Player/Animations/AM_Light_Attack_1.AM_Light_Attack_1"
        (:`then`
          (set `self.attackIndex` 1)
          (`KismetArrayLibrary.Array_Clear` (`self.Hit`))
          (goto _label :!via `Reset`))))))

(event `Sphere Trace`
  (bind _returnvalue (`SceneComponent.K2_GetComponentLocation` (`/Game/Assets/BluePrints/MainCharacter/BP_MainCharacter.AoETrace` (`self.Character_REF`))))
  ;[0.1594 1 0.332] Slam Sphere Trace
  (`KismetArrayLibrary.Array_Clear` (`self.Hit`))
  (bind _outhits (`KismetSystemLibrary.SphereTraceMultiForObjects` _returnvalue _returnvalue 300.0 (`self.Object Types`) false (`|MakeArray` null :!type "Actor Object Reference")))
  (for _array_element _outhits
    (bind (_bblockinghit _binitialoverlap _time _distance _location _impactpoint _normal _impactnormal _physmat _hitactor) (`GameplayStatics.BreakHitResult` _array_element))
    (bind _asbpidamage_recievers (cast `/Game/Assets/BluePrints/Interfaces/BPIDamageRecievers` _hitactor))
    (if (not (`KismetArrayLibrary.Array_Contains` (`self.Hit`) _asbpidamage_recievers))
      (message `/Game/Assets/BluePrints/Interfaces/BPIDamageRecievers.Knockback` _hitactor (`Actor.K2_GetActorLocation` (`self.Character_REF`)) 75.0 500.0)
      (message `/Game/Assets/BluePrints/Interfaces/BPIDamageRecievers.TakeDamage` _hitactor 20.0 5.0)
      (`KismetArrayLibrary.Array_Add` (`self.Hit`) _asbpidamage_recievers))))

(event `Light Hammer Attack`
  ;[0.1594 1 0.332] Combo System
  ;;[1 1 1] Function_Light Attack
  (set `self.Damage` 25.0)
  (set `self.Launch` 150.0)
  (set `self.Knockback` 300.0)
  (if (not (`self.isAttacking?`))
    (set `self.isAttacking?` true)
    (`self.Attack 1`)))

(event `Attack2`
  ;[0.1594 1 0.332] Combo System
  ;;[1 1 1] Anim_Light Attack Backhand
  (`/Engine/EditorBlueprintResources/StandardMacros.DoOnce` false :!label _label_2
    (:`Completed`
      (`self.SetHitboxVariables` (`KismetMathLibrary.MakeTransform` (250.0 0.0 0.0) (struct) (80.0 200.0 100.0)) (`KismetMathLibrary.MakeTransform` (100.0 0.0 0.0) (struct) (50.0 100.0 100.0)))
      (`|PlayMontage` (`self.carachterMesh`) "/Game/Assets/Animations/Player/Animations/AM_Light_Attack_2.AM_Light_Attack_2"
        (:`then`
          (set `self.attackIndex` 2)
          (`KismetArrayLibrary.Array_Clear` (`self.Hit`))
          (goto _label_2 :!via `Reset`))))))

(event `LightHammerAttack2`
  ;[0.1594 1 0.332] Combo System
  (`self.Attack2`)
  (set `self.secondAttack?` false))

(event `FollowUpAttack`
  ;[0.1594 1 0.332] Combo System
  ;;[1 1 1] Follow up Attack
  (`self.Light Attack Overhead`))

(event `SlashBoxTrace`
  (bind (_hitbox_variables_1_location _hitbox_variables_1_rotation _hitbox_variables_1_scale) (`KismetMathLibrary.BreakTransform` (`self.HitBox Variables_1`)))
  (bind (_hitbox_variables_2_location _hitbox_variables_2_rotation _hitbox_variables_2_scale) (`KismetMathLibrary.BreakTransform` (`self.HitBox Variables_2`)))
  (bind _slashhitarray (`self.SlashHitArray`))
  (bind _returnvalue (`SceneComponent.K2_GetComponentToWorld` (`Actor.RootComponent` (`self.Character_REF`))))
  (bind _returnvalue_2 (`KismetMathLibrary.TransformLocation` _returnvalue _hitbox_variables_2_location))
  (bind _returnvalue_3 (`KismetMathLibrary.TransformLocation` _returnvalue _hitbox_variables_1_location))
  ;[0.1594 1 0.332] Light Attack Trace
  (`KismetArrayLibrary.Array_Clear` (`self.Hit`))
  (`KismetArrayLibrary.Array_Clear` (`self.SlashHitArray`))
  (bind _outhits (`KismetSystemLibrary.BoxTraceMultiForObjects` :`Start` _returnvalue_3 :`End` _returnvalue_3 :`HalfSize` _hitbox_variables_1_scale :`Orientation` (`KismetMathLibrary.TransformRotation` _returnvalue _hitbox_variables_1_rotation) :`ObjectTypes` (`self.Object Types`) :`DrawTime` 0.5))
  (`KismetArrayLibrary.Array_Append` (`self.SlashHitArray`) _outhits)
  (bind _outhits_2 (`KismetSystemLibrary.BoxTraceMultiForObjects` :`Start` _returnvalue_2 :`End` _returnvalue_2 :`HalfSize` _hitbox_variables_2_scale :`Orientation` (`KismetMathLibrary.TransformRotation` _returnvalue _hitbox_variables_2_rotation) :`ObjectTypes` (`self.Object Types`) :`TraceColor` (struct :`R` 1.0 :`B` 0.526792 :`A` 1.0) :`TraceHitColor` (struct :`G` 1.0 :`B` 0.488338 :`A` 1.0) :`DrawTime` 0.5))
  (`KismetArrayLibrary.Array_Append` _slashhitarray _outhits_2)
  (for _array_element _slashhitarray
    (bind (_bblockinghit _binitialoverlap _time _distance _location _impactpoint _normal _impactnormal _physmat _hitactor) (`GameplayStatics.BreakHitResult` _array_element))
    (bind _asbpidamage_recievers (cast `/Game/Assets/BluePrints/Interfaces/BPIDamageRecievers` _hitactor))
    (bind _asbp_golem (cast `/Game/AI/EnemyFootsoldier/BP_Golem` _hitactor)
      (:`then`
        (set `self.ChargeAmmount` (`/Game/AI/EnemyFootsoldier/BP_Golem.ChargeAmount` _asbp_golem)))
      (:`CastFailed`
        (cast `/Game/AI/Turret/BP_Turret` _hitactor
          (:`then`
            (set `self.ChargeAmmount` 25.0))
          (:`CastFailed`
            (cast `/Game/AI/Bos/BP_BossMan` _hitactor
              (:`then`
                (set `self.ChargeAmmount` 20.0))
              (:`CastFailed`
                (bind _asbp_destructable (cast `/Game/Assets/Meshes/Props/Destrucatble/BP_Destructable` _hitactor))
                (set `self.ChargeAmmount` (`/Game/Assets/Meshes/Props/Destrucatble/BP_Destructable.ChargeAmmount` _asbp_destructable))))))))
    (if (not (`KismetArrayLibrary.Array_Contains` (`self.Hit`) _asbpidamage_recievers))
      (message `/Game/Assets/BluePrints/Interfaces/BPIDamageRecievers.Knockback` _hitactor (`Actor.K2_GetActorLocation` (`self.Character_REF`)) (`self.Knockback`) (`self.Launch`))
      (message `/Game/Assets/BluePrints/Interfaces/BPIDamageRecievers.TakeDamage` _hitactor (`self.Damage`) 3.0)
      (`/Game/Assets/BluePrints/MainCharacter/BP_MainCharacter.AddHammerCharge` (`self.Character_REF`) (`self.ChargeAmmount`))
      (`KismetArrayLibrary.Array_Add` (`self.Hit`) _asbpidamage_recievers))))

(event `Light Attack Overhead`
  ;[0.1594 1 0.332] Combo System
  ;;[1 1 1] Anim_Light Attack Overhead
  (`/Engine/EditorBlueprintResources/StandardMacros.DoOnce` false :!label _label_3
    (:`Completed`
      (`self.SetHitboxVariables` (`KismetMathLibrary.MakeTransform` (250.0 0.0 0.0) (struct) (80.0 80.0 150.0)) (`KismetMathLibrary.MakeTransform` (100.0 0.0 150.0) (struct) (80.0 40.0 80.0)))
      (`|PlayMontage` (`self.carachterMesh`) "/Game/Assets/Animations/HammerAttacks/AM_Overhead_Attack.AM_Overhead_Attack" 1.3
        (:`then`
          (set `self.attackIndex` 3)
          (`KismetArrayLibrary.Array_Clear` (`self.Hit`))
          (goto _label_3 :!via `Reset`))))))

(event `FollowUpAttackWindow`
  ;[0.1594 1 0.332] Combo System
  ;;[1 1 1] Timing window
  (set `self.secondAttack?` true)
  (`KismetSystemLibrary.Delay` 0.3)
  (set `self.secondAttack?` false))

(event `Stop Combo`
  ;[0.1594 1 0.332] Combo System
  ;;[1 1 1] Stop Combo/Attack
  (set `self.isAttacking?` false)
  (set `self.attackIndex` 0))

(event `Charge Attack`
  (bind _character_ref (`self.Character_REF`))
  ;[0.1594 1 0.332] Combo System
  ;;[1 1 1] Anim Spin Attack
  (`/Engine/EditorBlueprintResources/StandardMacros.DoOnce` false :!label _label_4
    (:`Completed`
      (`KismetSystemLibrary.Delay` 0.0)
      (`self.SetHitboxVariables` (`KismetMathLibrary.MakeTransform` (0.0 0.0 0.0) (struct) (160.0 160.0 150.0)) (`KismetMathLibrary.MakeTransform` (0.0 0.0 150.0) (struct) (160.0 160.0 80.0)))
      (set `/Game/Assets/BluePrints/MainCharacter/BP_MainCharacter.BlockInput?` true _character_ref)
      (set `self.isSpinning?` true)
      (`|PlayMontage` (`self.carachterMesh`) "/Game/Assets/Animations/Player/Animations/AM_DashAttackSpin.AM_DashAttackSpin"
        (:`then`
          (`KismetArrayLibrary.Array_Clear` (`self.Hit`))
          (goto _label_4 :!via `Reset`))
        (:`OnCompleted`
          (set `self.isSpinning?` false))
        (:`OnBlendOut`
          (set `/Game/Assets/BluePrints/MainCharacter/BP_MainCharacter.BlockInput?` false _character_ref :!label _label_5))
        (:`OnInterrupted`
          (`self.Stop Combo`)
          (goto _label_5))))))

(event `Heavy Hammer Attack`
  ;[0.1594 1 0.332] Combo System
  ;;[1 1 1] Function_Charge Attack
  (if (`self.isSlamming?`)
    _
    (elif (not (`self.isAttacking?`))
      (set `self.isAttacking?` true)
      (set `self.Damage` 50.0)
      (set `self.Knockback` 1000.0)
      (set `self.Launch` 500.0)
      (`self.Charge Attack`))))

(event `SetHitboxVariables`
  (params (Transform_1 :type "Transform Structure") (Transform_2 :type "Transform Structure"))
  ;[0.1594 1 0.332] Light Attack Trace
  (set `self.HitBox Variables_1` Transform_1)
  (set `self.HitBox Variables_2` Transform_2))

(event `SlamAttack`
  (bind _character_ref (`self.Character_REF`))
  ;[1 1 1] Slam Attack
  (if (not (`self.isSlamming?`))
    (set `self.isSlamming?` true)
    (`/Game/Assets/BluePrints/MainCharacter/BP_MainCharacter.LaunchBackDown` _character_ref 0.0)
    (`Character.PlayAnimMontage` _character_ref "/Game/Assets/Animations/Player/Animations/AM_Groundslam.AM_Groundslam" 0.75 "None")
    (`self.Stop Combo`)
    (set `self.isSlamming?` false)))

(event `Play Rupture Effect`
  (bind _character_ref (`self.Character_REF`))
  (bind (_returnvalue_x _returnvalue_y _returnvalue_z) (`KismetMathLibrary.BreakVector` (`Actor.K2_GetActorLocation` _character_ref)))
  (bind (_returnvalue_x_2 _returnvalue_y_2) (`KismetMathLibrary.BreakVector` (* (`Actor.GetActorForwardVector` _character_ref) 100.0)))
  (bind (_returnvalue_x_3 _returnvalue_y_3) (`KismetMathLibrary.BreakVector` (+ (`SceneComponent.K2_GetComponentLocation` (`/Game/Assets/BluePrints/MainCharacter/BP_MainCharacter.HammerBottomPoint` _character_ref)) (`KismetMathLibrary.MakeVector` _returnvalue_x_2 _returnvalue_y_2))))
  ;[1 1 1] Spell_Rupture
  (bind _returnvalue (`GameplayStatics.GetActorOfClass` "/Game/Assets/BluePrints/BP_Spells/BaseClass/BP_Rupture_Child.BP_Rupture_Child_C"))
  (message `/Game/Assets/BluePrints/BP_Spells/BaseClass/BPI_SpellEffects.CastSpell` _returnvalue (0.0 0.0 0.0) (`Actor.K2_GetActorRotation` _character_ref) null (`KismetMathLibrary.MakeVector` _returnvalue_x_3 _returnvalue_y_3 (- _returnvalue_z 100.0)) 0.0))

(event `Hammer Trace Loop`
  ;[0.159 1 0.3325] Hammer Trace
)

(event `Start Hammer Trace`
  ;[0.159 1 0.3325] Hammer Trace
)

(event `Stop Hammer Trace`
  ;[0.159 1 0.3325] Hammer Trace
)