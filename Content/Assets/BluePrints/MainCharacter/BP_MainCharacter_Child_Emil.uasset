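; BP_MainCharacter_Child_Emil is a main character child Blueprint that adds an aim focus camera with a crosshair.
; BeginPlay stores the boom length and creates the crosshair widget.
; IA_Focus plays or reverses a timeline that lerps boom offset and length, calling AddToViewport every update, so reversing re-adds the crosshair removed on release.
; Hammer throw and recall logic is present but unconnected.
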(event `self.ReceiveBeginPlay`
  (`parent.ReceiveBeginPlay`)
  (set `self.BoomStartLength` (`SpringArmComponent.TargetArmLength` (`self.CameraBoom`)))
  (bind _returnvalue (`|CreateWidget` "/Game/Assets/UI/HUD_Widgets/WBP_Crosshair.WBP_Crosshair_C"))
  (set `self.Crosshair_REF_0` _returnvalue))

(event `EnhancedInput|/Game/Assets/Input/Actions/IA_Focus`
  (params (ActionValue :type Boolean) (ElapsedSeconds :type "Float (double-precision)") (TriggeredSeconds :type "Float (double-precision)") (InputAction :type "InputAction Object Reference" :default "/Game/Assets/Input/Actions/IA_Focus.IA_Focus"))
  (bind _crosshair_ref_0 (`self.Crosshair_REF_0`))
  (bind _cameraboom (`self.CameraBoom`))
  (:`Started`
    (bind (_direction _focus_time) (`Timeline|Timeline_0` :!label _label)
      (:`Update`
        (set `SpringArmComponent.SocketOffset` (`KismetMathLibrary.VLerp` (`self.CameraBoomStartOffset`) (`self.CameraBoomFocusOffset`) _focus_time) _cameraboom)
        (set `SpringArmComponent.TargetArmLength` (`KismetMathLibrary.Lerp` (`self.BoomStartLength`) (`self.BoomFocusLength`) _focus_time) _cameraboom)
        (`UserWidget.AddToViewport` _crosshair_ref_0 0))))
  (:`Completed`
    (`Widget.RemoveFromParent` _crosshair_ref_0)
    (goto _label :!via `ReverseFromEnd`)))

(event `EnhancedInput|/Game/Assets/Input/Actions/IA_Throw`
  (params (ActionValue :type Boolean) (ElapsedSeconds :type "Float (double-precision)") (TriggeredSeconds :type "Float (double-precision)") (InputAction :type "InputAction Object Reference" :default "/Game/Assets/Input/Actions/IA_Throw.IA_Throw")))

(fn `UserConstructionScript`
  (`parent.UserConstructionScript`))