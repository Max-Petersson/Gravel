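; Thrown hammer projectile that bounces off the first thing it hits and can be recalled to the player's hand.
; A Tick sphere trace stops flight, then a timeline spins it along a spline arc to a random traced landing point, ending in a Niagara effect.
; Recall rebuilds a sideways-curved spline to the moving hand each tick, then restores throwing and destroys the actor.
; Overlaps send knockback and zero-damage messages once per target, resetting on recall.
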(event `SetSpline Types`
  (bind _bouncepath (`self.BouncePath`))
  (`SplineComponent.SetSplinePointType` _bouncepath 0 "CurveClamped" true)
  (`SplineComponent.SetSplinePointType` _bouncepath 1 "CurveCustomTangent" true)
  (`SplineComponent.SetSplinePointType` _bouncepath 2 "CurveClamped" true))

(event `self.ReceiveBeginPlay`)

(event `self.ReceiveTick`
  (params (DeltaSeconds :type "Float (single-precision)"))
  (bind _return_start_value (`self.Return Start Value`))
  (bind _returnvalue (`SceneComponent.K2_GetComponentLocation` (`self.CollisionPoint`)))
  (bind (_returnvalue_location _returnvalue_rotation) (`KismetMathLibrary.BreakTransform` (`SceneComponent.K2_GetComponentToWorld` (`/Game/Assets/BluePrints/MainCharacter/BP_MainCharacter.HammerMidPoint` (`self.Character`)))))
  (`|ExecutionSequence`
    (:`then_0`
      (bind (_outhit _returnvalue_2) (`KismetSystemLibrary.SphereTraceSingle` _returnvalue _returnvalue 25.0 "TraceTypeQuery1" false (`|MakeArray` (`GameplayStatics.GetPlayerCharacter` 0) :!type "Actor Object Reference")))
      (if _returnvalue_2
        (`/Engine/EditorBlueprintResources/StandardMacros.DoOnce` false
          (:`Completed`
            (cast `/Game/Assets/BluePrints/Dummies/BP_Dummy` (`.HitActor` (`GameplayStatics.BreakHitResult` _outhit))
              (:`then`
                (`MovementComponent.StopMovementImmediately` (`self.ProjectileMovement`))
                (set `RotatingMovementComponent.RotationRate` (struct) (`self.RotatingMovement`))
                (set `ProjectileMovementComponent.ProjectileGravityScale` 0.0 (`self.ProjectileMovement`))
                (`KismetSystemLibrary.PrintString` "Hit Enemy")
                (`self.BounceEffect`))
              (:`CastFailed`
                (`MovementComponent.StopMovementImmediately` (`self.ProjectileMovement`))
                (set `RotatingMovementComponent.RotationRate` (struct) (`self.RotatingMovement`))
                (set `ProjectileMovementComponent.ProjectileGravityScale` 0.0 (`self.ProjectileMovement`))
                (`KismetSystemLibrary.PrintString` "Nothing Here")
                (`self.BounceEffect`)))))))
    (:`then_1`
      (if (`self.UpdateReturnSpline`)
        (set `self.Hand Rotation` _returnvalue_rotation)
        (`SplineComponent.SetSplinePoints` (`self.BouncePath`) (`|MakeArray` _return_start_value (+ (/ (+ _return_start_value _returnvalue_location) 2.0) (* (`self.GetActorRightVector` (`self.Character`)) 200.0)) _returnvalue_location) "World" true)
        (`self.SetSpline Types`)))))

(event `BounceEffect`
  (bind _start_rotation (`self.Start Rotation`))
  (bind _returnvalue (`SceneComponent.K2_GetComponentLocation` (`self.TopPoint`)))
  (bind (_origin _boxextent) (`KismetSystemLibrary.GetComponentBounds` (`self.LandingBox`)))
  (bind (_x _y _z) (`KismetMathLibrary.BreakVector3f` _returnvalue))
  (bind _returnvalue_2 (`KismetMathLibrary.RandomPointInBoundingBox` _origin _boxextent))
  (bind (_returnvalue_x _returnvalue_y) (`KismetMathLibrary.BreakVector` (`KismetMathLibrary.GetDirectionUnitVector` _returnvalue (`SceneComponent.K2_GetComponentLocation` (`self.Hammer`)))))
  (bind _returnvalue_3 (`KismetMathLibrary.Normal` (`KismetMathLibrary.MakeVector` _returnvalue_x _returnvalue_y)))
  (bind _outhit (`KismetSystemLibrary.LineTraceSingle` _returnvalue_2 (+ _returnvalue_2 (0.0 0.0 -1000.0)) "TraceTypeQuery1" false (`|MakeArray` (`self.Character`) :!type "Actor Object Reference")))
  (bind (_bblockinghit _binitialoverlap _time _distance _location _impactpoint) (`GameplayStatics.BreakHitResult` _outhit))
  (set `self.Bounce Landing Point` _impactpoint)
  (bind _returnvalue_4 (+ _impactpoint (0.0 0.0 20.0)))
  (bind (_returnvalue_x_2 _returnvalue_y_2) (`KismetMathLibrary.BreakVector` (`KismetMathLibrary.GetDirectionUnitVector` _returnvalue _returnvalue_4)))
  (bind _returnvalue_5 (`KismetMathLibrary.Normal` (`KismetMathLibrary.MakeVector` _returnvalue_x_2 _returnvalue_y_2)))
  (bind _returnvalue_6 (`KismetMathLibrary.DegAcos` (`KismetMathLibrary.Dot_VectorVector` _returnvalue_5 _returnvalue_3)))
  (bind (_returnvalue_x_3 _returnvalue_y_3 _returnvalue_z) (`KismetMathLibrary.BreakVector` (`KismetMathLibrary.Cross_VectorVector` _returnvalue_5 _returnvalue_3)))
  (set `self.Landing Angle` (`KismetMathLibrary.SelectFloat` (* _returnvalue_6 -1.0) _returnvalue_6 (> _returnvalue_z 0.0)))
  (bind (_returnvalue_x_4 _returnvalue_y_4) (`KismetMathLibrary.BreakVector` (/ (+ _returnvalue _returnvalue_4) 2)))
  (bind (_x_2 _y_2 _z_2) (`KismetMathLibrary.BreakVector3f` _returnvalue_4))
  ;[0.05098 0.05098 0.05098] Sets Start, Mid, End point for spline
  (`SplineComponent.SetSplinePoints` (`self.BouncePath`) (`|MakeArray` _returnvalue (+ (`KismetMathLibrary.MakeVector` _returnvalue_x_4 _returnvalue_y_4) (`KismetMathLibrary.MakeVector` 0.0 0.0 (+ (`KismetMathLibrary.SelectFloat` _z _z_2 (> _z _z_2)) 150.0))) _returnvalue_4) "World" true)
  (`self.SetSpline Types`)
  (set `self.Start Rotation` (`SceneComponent.K2_GetComponentRotation` (`self.TopPoint`)))
  (bind (_direction _bouncetime _spinnnnntime) (`Timeline|BounceTimeline` :!via `PlayFromStart` :!label _label)
    (:`Update`
      (`self.Move Along Spline` _bouncetime (`self.TopPoint`) _start_rotation (`KismetMathLibrary.MakeRotator` (+ (`self.Landing Angle`) 90.0) 630.0 (.yaw _start_rotation)) _spinnnnntime))
    (:`Finished`
      (`NiagaraFunctionLibrary.SpawnSystemAtLocation` "/Game/Assets/VFX/MovementVFX/NS_Rupturetest.NS_Rupturetest" (`self.Bounce Landing Point`)))))

(event `CancelBounce`
  (goto _label :!via `Stop`))

(event `Recall Hammer`
  (`/Engine/EditorBlueprintResources/StandardMacros.DoOnce` false
    (:`Completed`
      (`self.CancelBounce`)
      (`KismetArrayLibrary.Array_Clear` (`self.Damagable`))
      (bind _asbp_main_character (cast `/Game/Assets/BluePrints/MainCharacter/BP_MainCharacter` (`GameplayStatics.GetPlayerCharacter` 0)))
      (set `self.Character` _asbp_main_character)
      (set `self.Return Start Value` (`SceneComponent.K2_GetComponentLocation` (`self.TopPoint`)))
      (set `self.UpdateReturnSpline` true)
      (`TimelineComponent.SetPlayRate` (`self.ReturnTimeline`) (`self.Return Speed Modifier`))
      (set `self.Start Rotation` (`SceneComponent.K2_GetComponentRotation` (`self.TopPoint`)))
      (bind (_direction _move_track) (`Timeline|ReturnTimeline` :!via `PlayFromStart`)
        (:`Update`
          (`self.Move Along Spline` _move_track (`self.TopPoint`) (`self.Start Rotation`) (`KismetMathLibrary.MakeRotator` (+ (.roll (`self.Hand Rotation`)) 360.0) (.pitch (`self.Hand Rotation`)) (.yaw (`self.Hand Rotation`))) _move_track))
        (:`Finished`
          (`SceneComponent.SetVisibility` (`/Game/Assets/BluePrints/MainCharacter/BP_MainCharacter.SK Blunt Crude Hammer` (`self.Character`)) true false)
          (set `/Game/Assets/BluePrints/MainCharacter/BP_MainCharacter.Can Throw?` true (`self.Character`))
          (`self.K2_DestroyActor`))))))

(event `self.CollisionPoint.OnComponentBeginOverlap`
  (params (OverlappedComponent :type "PrimitiveComponent Object Reference") (OtherActor :type "Actor Object Reference") (OtherComp :type "PrimitiveComponent Object Reference") (OtherBodyIndex :type Integer) (bFromSweep :type Boolean) (SweepResult :type "HitResult Structure (by ref)"))
  (bind _asbpidamage_recievers (cast `/Game/Assets/BluePrints/Interfaces/BPIDamageRecievers` OtherActor))
  (if (not (`KismetArrayLibrary.Array_Contains` (`self.Damagable`) _asbpidamage_recievers))
    (`KismetArrayLibrary.Array_Add` (`self.Damagable`) _asbpidamage_recievers)
    (bind _returnvalue (`KismetSystemLibrary.Conv_InterfaceToObject` _asbpidamage_recievers))
    (message `/Game/Assets/BluePrints/Interfaces/BPIDamageRecievers.Knockback` _returnvalue (`self.K2_GetActorLocation`) 5.0 500.0)
    (message `/Game/Assets/BluePrints/Interfaces/BPIDamageRecievers.TakeDamage` _returnvalue 0.0)))

(fn `Move Along Spline`
  (params (MoveAlpha :type "Float (single-precision)") (`Moved Target` :type "ArrowComponent Object Reference") (Rot_Original :type "Rotator Structure") (`Rot End` :type "Rotator Structure") (RotAlpha :type "Float (single-precision)"))
  (`SceneComponent.K2_SetRelativeLocation` `Moved Target` (`SplineComponent.GetLocationAtTime` (`self.BouncePath`) MoveAlpha "Local" false) false false)
  (`SceneComponent.K2_SetWorldRotation` `Moved Target` (`KismetMathLibrary.RLerp` Rot_Original `Rot End` RotAlpha) false false))

(fn `UserConstructionScript`)