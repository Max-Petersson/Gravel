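; Combust variant of a throwable hammer weapon that adds an explosion as its spell effect.
; TriggerSpell spawns BP_ExplosionEffect at the Hammer component's world location.
; BeginPlay, overlap handling and construction only call the parent, so all other behavior is inherited.
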(event `self.ReceiveBeginPlay`
  (`parent.ReceiveBeginPlay`))

(event `self.ReceiveActorBeginOverlap`
  (params (OtherActor :type "Actor Object Reference"))
  (`parent.ReceiveActorBeginOverlap` OtherActor))

(event `/Game/Assets/BluePrints/Interfaces/BPI_HammerSpells.Trigger Spell`
  (`|SpawnActorFromClass` "/Game/Assets/BluePrints/BP_Spells/Combustion/BP_ExplosionEffect.BP_ExplosionEffect_C" (`KismetMathLibrary.MakeTransform` (`SceneComponent.K2_GetComponentLocation` (`self.Hammer`))) "Undefined" "OverrideRootScale" null null))

(fn `UserConstructionScript`
  (`parent.UserConstructionScript`))