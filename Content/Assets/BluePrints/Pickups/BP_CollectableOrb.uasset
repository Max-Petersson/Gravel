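; A healing orb pickup that hovers and spins on a timeline until the main character overlaps it.
; The first overlap stops the hover, removes the orb's mesh and effects, heals through the player's health component and plays a sound.
; It then activates homing Niagara particles, with Tick feeding the player's HP crystal position into their aim variable until the actor destroys itself after a short delay.
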(event `self.Sphere Collision.OnComponentBeginOverlap`
  (params (OverlappedComponent :type "PrimitiveComponent Object Reference") (OtherActor :type "Actor Object Reference") (OtherComp :type "PrimitiveComponent Object Reference") (OtherBodyIndex :type Integer) (bFromSweep :type Boolean) (SweepResult :type "HitResult Structure (by ref)"))
  (bind _asbp_main_character (cast `/Game/Assets/BluePrints/MainCharacter/BP_MainCharacter` OtherActor))
  (bind _output_get (set `self.Player` _asbp_main_character))
  (`/Engine/EditorBlueprintResources/StandardMacros.DoOnce` false
    (:`Completed`
      (`self.StopHovering`)
      (`ActorComponent.K2_DestroyComponent` (`self.NS_OrbEffects`))
      (`ActorComponent.K2_DestroyComponent` (`self.Mesh`))
      (`/Game/Assets/BluePrints/BPC_HealthSystem.IncreaseHealth` (`/Game/Assets/BluePrints/MainCharacter/BP_MainCharacter.BPC_HealthSystem` _output_get) 5.0)
      (`GameplayStatics.PlaySound2D` "/Game/SoundFX/MetaSounds/Implemented/MS_HealPickup.MS_HealPickup" 1.0 1.0 0.0 null null)
      (`ActorComponent.Activate` (`self.NS_HomingParticles`) false)
      (set `self.Start?` true)
      (`KismetSystemLibrary.Delay` 1.0)
      (`self.K2_DestroyActor`))))

(event `self.ReceiveTick`
  (params (DeltaSeconds :type "Float (single-precision)"))
  (if (`self.Start?`)
    (`NiagaraComponent.SetVariableVec3` (`self.NS_HomingParticles`) "Aim_Position" (`SceneComponent.K2_GetComponentLocation` (`/Game/Assets/BluePrints/MainCharacter/BP_MainCharacter.HPCrystal_2` (`self.Player`))))))

(event `self.ReceiveBeginPlay`
  (bind (_direction _newtrack_0) (`Timeline|Hovering` :!label _label)
    (:`Update`
      (`SceneComponent.K2_AddWorldOffset` (`self.Base`) _newtrack_0 false false)
      (`SceneComponent.K2_AddWorldRotation` (`self.Mesh`) (struct :`Yaw` 1.0) false false))))

(event `StopHovering`
  (goto _label :!via `Stop`))

(fn `UserConstructionScript`)