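; BP_Notification is a trigger box that shows an on-screen tutorial message while BP_MainCharacter stands inside it.
; On overlap, a DoOnce gate creates a WBP_JumpTutorial widget, fills it with the formatted TextToDisplay and adds it to the viewport.
; On exit, a retriggerable half-second delay rechecks the inside flag, so a quick re-entry keeps the message; otherwise it removes the notification and resets the gate.
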(event `self.Box.OnComponentBeginOverlap`
  (params (OverlappedComponent :type "PrimitiveComponent Object Reference") (OtherActor :type "Actor Object Reference") (OtherComp :type "PrimitiveComponent Object Reference") (OtherBodyIndex :type Integer) (bFromSweep :type Boolean) (SweepResult :type "HitResult Structure (by ref)"))
  (cast `/Game/Assets/BluePrints/MainCharacter/BP_MainCharacter` OtherActor)
  (set `self.PlayInside?` true)
  (`/Engine/EditorBlueprintResources/StandardMacros.DoOnce` false :!label _label
    (:`Completed`
      (bind _returnvalue (`|CreateWidget` "/Game/Assets/UI/HUD_Notifications/WBP_JumpTutorial.WBP_JumpTutorial_C" (`GameplayStatics.GetPlayerController` 0)))
      (`/Game/Assets/UI/HUD_Notifications/WBP_JumpTutorial.Set text` _returnvalue (`|FormatText` (`self.TextToDisplay`) " \n"))
      (`UserWidget.AddToViewport` _returnvalue 0))))

(event `self.Box.OnComponentEndOverlap`
  (params (OverlappedComponent :type "PrimitiveComponent Object Reference") (OtherActor :type "Actor Object Reference") (OtherComp :type "PrimitiveComponent Object Reference") (OtherBodyIndex :type Integer))
  (cast `/Game/Assets/BluePrints/MainCharacter/BP_MainCharacter` OtherActor)
  (bind _output_get (set `self.PlayInside?` false))
  (`KismetSystemLibrary.RetriggerableDelay` 0.5)
  (if (not _output_get)
    (`/Engine/EditorBlueprintResources/StandardMacros.IsValid` (stale `self.Box.OnComponentBeginOverlap` _returnvalue)
      (:`Is Valid`
        (`/Game/Assets/UI/HUD_Notifications/WBP_JumpTutorial.RemoveNotify` (stale `self.Box.OnComponentBeginOverlap` _returnvalue))
        (goto _label :!via `Reset`)))))

(fn `UserConstructionScript`)