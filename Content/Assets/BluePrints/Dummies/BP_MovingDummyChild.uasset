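; Walkable training dummy child Blueprint that wanders the level and triggers its own replacement when destroyed.
; Two seconds after BeginPlay it starts RandomRoam, which uses AI MoveTo toward random reachable points nearby.
; Roaming repeats after a short random pause only when a move succeeds, so a failed move ends it.
; On Destroyed it asks BP_DummySpawner to spawn another walkable dummy; knockback direction simply defers to the parent.
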(event `self.ReceiveDestroyed`
  (bind _returnvalue (`GameplayStatics.GetActorOfClass` "/Game/Assets/BluePrints/Dummies/BP_DummySpawner.BP_DummySpawner_C"))
  (`/Game/Assets/BluePrints/Dummies/BP_DummySpawner.SpawnWalkableDummy` _returnvalue))

(event `self.ReceiveBeginPlay`
  (`KismetSystemLibrary.Delay` 2.0)
  (`self.RandomRoam`)
  (`KismetSystemLibrary.PrintString` "Hello"))

(event `RandomRoam`
  ;[1 1 1] Move to random location
  (`|AIMoveTo` self (`NavigationSystemV1.K2_GetRandomReachablePointInRadius` (`self.K2_GetActorLocation`) 2500.0 null null) null
    (:`OnSuccess`
      (`KismetSystemLibrary.Delay` (`KismetMathLibrary.RandomFloatInRange` 2.0 4.0))
      (`self.RandomRoam`))))

(fn `Calculate KB Dir`
  (params (`Knockback Source` :type "Vector Structure") (`My Position` :type "Vector Structure") (`Directional Strenght` :type "Float (double-precision)") (`Launch Strenght` :type "Float (double-precision)"))
  (returns (`Applied Knockback` :type "Vector Structure"))
  (bind _applied_knockback (`parent.Calculate KB Dir` `Knockback Source` `My Position` `Directional Strenght` `Launch Strenght`))
  (return _applied_knockback))

(fn `UserConstructionScript`
  (`parent.UserConstructionScript`))