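; BP_Turret is a stationary enemy that rises from the ground via a timeline and registers with BP_WaveManager until destroyed.
; Once risen, it traces for the player each tick, turns toward them when visible, and triggers a delayed rock throw.
; After a windup effect, it spawns an AoE indicator at a trace hit from the player, unless Knockback cancels it during the stun window.
; The projectile-shot branch is disconnected.
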(event `self.ReceiveDestroyed`
  (bind _returnvalue (`GameplayStatics.GetActorOfClass` "/Game/AI/WaveLogic/BP_WaveManager.BP_WaveManager_C"))
  (`/Engine/EditorBlueprintResources/StandardMacros.IsValid` _returnvalue
    (:`Is Valid`
      (`/Engine/EditorBlueprintResources/StandardMacros.DoOnce` false
        (:`Completed`
          (`/Game/AI/WaveLogic/BP_WaveManager.SubtractFromNeeded` _returnvalue))))))

(event `self.ReceiveBeginPlay`
  (bind _asbp_main_character (cast `/Game/Assets/BluePrints/MainCharacter/BP_MainCharacter` (`GameplayStatics.GetPlayerCharacter` 0)))
  (set `self.As BP Main Character` _asbp_main_character)
  (bind _returnvalue (`GameplayStatics.GetActorOfClass` "/Game/AI/WaveLogic/BP_WaveManager.BP_WaveManager_C"))
  (`/Engine/EditorBlueprintResources/StandardMacros.IsValid` _returnvalue
    (:`Is Valid`
      (`/Game/AI/WaveLogic/BP_WaveManager.AddToNeeded` _returnvalue))
    (:`Is Not Valid`
      _))
  (`SceneComponent.K2_SetRelativeLocation` (`self.Mesh`) (0.0 0.0 -120.0) false false)
  (`KismetSystemLibrary.Delay` (`KismetMathLibrary.RandomFloatInRange` 0.5 1.0))
  (bind (_direction _rising_effect) (`Timeline|Rising`)
    (:`Update`
      (`SceneComponent.K2_SetRelativeLocation` (`self.Mesh`) (`KismetMathLibrary.MakeVector` 0.0 0.0 _rising_effect) false false))
    (:`Finished`
      (set `self.Intro` false))
    (:`Crack`
      (`NiagaraFunctionLibrary.SpawnSystemAtLocation` "/Game/Assets/VFX/MovementVFX/NS_Rupturetest.NS_Rupturetest" (- (`self.K2_GetActorLocation`) (0.0 0.0 130.0))))))

(event `self.ReceiveTick`
  (params (DeltaSeconds :type "Float (single-precision)"))
  (bind (_returnvalue_roll _returnvalue_pitch _returnvalue_yaw) (`KismetMathLibrary.BreakRotator` (`KismetMathLibrary.RInterpTo` (`self.K2_GetActorRotation`) (`KismetMathLibrary.FindLookAtRotation` (`self.K2_GetActorLocation`) (`self.K2_GetActorLocation` (`self.As BP Main Character`))) (`GameplayStatics.GetWorldDeltaSeconds`))))
  (if (not (`self.Intro`))
    (bind _outhit (`KismetSystemLibrary.LineTraceSingle` (+ (`self.K2_GetActorLocation`) (0.0 0.0 100.0)) (+ (`self.K2_GetActorLocation` (`self.As BP Main Character`)) (0.0 0.0 50.0)) "TraceTypeQuery1"))
    (bind _output_get (set `self.Sees Player?` (== (`self.As BP Main Character`) (`.HitActor` (`GameplayStatics.BreakHitResult` _outhit)))))
    (if _output_get
      (`self.K2_SetActorRotation` (`KismetMathLibrary.MakeRotator` 0.0 0.0 _returnvalue_yaw))
      (`self.ThrowRock`))))

(event `/Game/Assets/BluePrints/Interfaces/BPIDamageRecievers.Knockback`
  (params (KnockbackSource :type "Vector Structure") (KnockbackValue :type "Float (double-precision)") (`Launch Value` :type "Float (double-precision)"))
  (bind _niagravis (`self.NiagraVis`))
  (if (`self.Can Fire?`)
    (set `self.Can Fire?` false)
    (if (`KismetSystemLibrary.IsValid` _niagravis)
      (`ActorComponent.K2_DestroyComponent` _niagravis))))

(event `/Game/Assets/BluePrints/Interfaces/BPIDamageRecievers.TakeDamage`
  (params (`Damage Taken` :type "Float (double-precision)"))
  (set `self.Health` (- (`self.Health`) `Damage Taken`))
  (if (<= (`self.Health`) 0.0)
    (`self.K2_DestroyActor`)))

(event `ThrowRock`
  (`KismetSystemLibrary.Delay` (`KismetMathLibrary.RandomFloatInRange` 5.0 6.0))
  (if (`self.Sees Player?`)
    (bind _returnvalue (`NiagaraFunctionLibrary.SpawnSystemAtLocation` "/Game/Assets/VFX/SpellVFX/NS_StoneThrow.NS_StoneThrow" (`SceneComponent.K2_GetComponentLocation` (`self.Spawner`))))
    (set `self.NiagraVis` _returnvalue)
    (`KismetSystemLibrary.PrintString` "windup")
    (set `self.Can Fire?` true)
    (`KismetSystemLibrary.Delay` 2.0) ; This is the stun window
    (if (`self.Can Fire?`)
      (`self.SpawnExplosion`))
    (else
      (set `self.Can Fire?` true))))

(event `SpawnExplosion`
  (bind _returnvalue (`self.K2_GetActorLocation` (`self.As BP Main Character`)))
  (bind _outhit (`KismetSystemLibrary.LineTraceSingle` _returnvalue (* (* _returnvalue (`KismetMathLibrary.Vector_Down`)) 200.0) "TraceTypeQuery1" false (`|MakeArray` (`self.As BP Main Character`) :!type "Actor Object Reference")))
  (`|SpawnActorFromClass` "/Game/Assets/BluePrints/Dummies/BP_IndicatorForAoe.BP_IndicatorForAoe_C" (`KismetMathLibrary.MakeTransform` (`.ImpactPoint` (`GameplayStatics.BreakHitResult` _outhit))) "Undefined" "OverrideRootScale" self null)
  (`ActorComponent.K2_DestroyComponent` (`self.NiagraVis`)))

(fn `UserConstructionScript`
  (`parent.UserConstructionScript`))