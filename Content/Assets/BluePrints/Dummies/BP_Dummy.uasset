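; BP_Dummy is a launchable character that acts as a damageable dummy.
; TakeDamage subtracts from Health and destroys the actor at zero or below.
; Knockback launches it with both velocity overrides, using CalculateKBDir to combine a separate vertical strength with a horizontal push away from the source.
; The horizontal offset is not normalized, so push strength grows with distance from the source.
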(event `/Game/Assets/BluePrints/Interfaces/BPIDamageRecievers.TakeDamage`
  (params (`Damage Taken` :type "Float (double-precision)"))
  (set `self.Health` (- (`self.Health`) `Damage Taken`))
  (if (<= (`self.Health`) 0.0)
    (`self.K2_DestroyActor`)))

(event `/Game/Assets/BluePrints/Interfaces/BPIDamageRecievers.Knockback`
  (params (KnockbackSource :type "Vector Structure") (KnockbackValue :type "Float (double-precision)") (`Launch Value` :type "Float (double-precision)"))
  (bind _applied_knockback (`self.Calculate KB Dir` KnockbackSource (`self.K2_GetActorLocation`) KnockbackValue `Launch Value`))
  (`self.LaunchCharacter` _applied_knockback true true))

(fn `Calculate KB Dir`
  (params (`Knockback Source` :type "Vector Structure") (`My Position` :type "Vector Structure") (`Directional Strenght` :type "Float (double-precision)") (`Launch Strenght` :type "Float (double-precision)"))
  (returns (`Applied Knockback` :type "Vector Structure"))
  (locals (KBS :type "Vector Structure") (MYPOS :type "Vector Structure") (KnockbackDirection :type "Vector Structure"))
  (bind (_kbs_x _kbs_y _kbs_z) (`KismetMathLibrary.BreakVector` (`local.KBS`)))
  (bind (_mypos_x _mypos_y _mypos_z) (`KismetMathLibrary.BreakVector` (`local.MYPOS`)))
  (set `local.KBS` `Knockback Source`)
  (set `local.MYPOS` `My Position`)
  (bind _output_get (set `local.KnockbackDirection` (+ (`KismetMathLibrary.MakeVector` 0.0 0.0 `Launch Strenght`) (* `Directional Strenght` (- (- (`local.MYPOS`) (`KismetMathLibrary.MakeVector` 0.0 0.0 _mypos_z)) (- (`local.KBS`) (`KismetMathLibrary.MakeVector` 0.0 0.0 _kbs_z)))))))
  (return _output_get))

(fn `UserConstructionScript`)