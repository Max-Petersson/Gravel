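; Anim notify state that opens and closes the hammer melee trace window on the main character during an animation.
; On notify begin it casts the mesh owner to BP_MainCharacter and calls StartHammerTrace on its BPCHammerMeleeSystem component.
; On notify end it makes the same cast and calls StopHammerTrace, so the notify's span on the timeline sets when the trace is active.
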(fn `Received_NotifyBegin`
  (params (MeshComp :type "SkeletalMeshComponent Object Reference") (Animation :type "AnimSequenceBase Object Reference") (TotalDuration :type "Float (single-precision)") (EventReference :type "AnimNotifyEventReference Structure (by ref)"))
  (returns (ReturnValue :type Boolean))
  (bind _asbp_main_character (cast `/Game/Assets/BluePrints/MainCharacter/BP_MainCharacter` (`ActorComponent.GetOwner` MeshComp)))
  (`/Game/Assets/BluePrints/Erik/BPC_HammerMeleeSystem.Start Hammer Trace` (`/Game/Assets/BluePrints/MainCharacter/BP_MainCharacter.BPC_HammerMeleeSystem` _asbp_main_character))
  (return false))

(fn `Received_NotifyEnd`
  (params (MeshComp :type "SkeletalMeshComponent Object Reference") (Animation :type "AnimSequenceBase Object Reference") (EventReference :type "AnimNotifyEventReference Structure (by ref)"))
  (returns (ReturnValue :type Boolean))
  (bind _asbp_main_character (cast `/Game/Assets/BluePrints/MainCharacter/BP_MainCharacter` (`ActorComponent.GetOwner` MeshComp)))
  (`/Game/Assets/BluePrints/Erik/BPC_HammerMeleeSystem.Stop Hammer Trace` (`/Game/Assets/BluePrints/MainCharacter/BP_MainCharacter.BPC_HammerMeleeSystem` _asbp_main_character))
  (return false))