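; Component on the main character that runs hammer melee: light attack with timed overhead follow-up, heavy charge attack and launching slam.
; Attack events set damage and knockback values and play montages.
; A fast looping timer sphere-traces along the hammer head, sending damage and knockback through BPIDamageRecievers, with a Hit list preventing repeat hits.
; Separate events deliver a radial AoE hit and cast the Rupture effect ahead of the hammer.
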(event `self.ReceiveBeginPlay`
  (bind _asbp_main_character (cast `/Game/Assets/BluePrints/MainCharacter/BP_MainCharacter` (`self.GetOwner`)))
  (set `self.Character_REF` _asbp_main_character)
  (set `self.carachterMesh` (`Character.Mesh` _asbp_main_character)))

(event `Attack 2`
  ;[1 1 1] Attack 2
)

(event `Light Attack`
  ;[0.1594 1 0.332] Combo System
  ;;[1 1 1] Attack Input
  (if (`self.isSlamming?`)
    _
    (elif (`self.canAttack?`)
      (if (`self.secondAttack?`)
        (`self.FollowUpAttack`)
        (else
          (`self.Light Hammer Attack`))))))

(event `Attack 1`
  ;[0.1594 1 0.332] Combo System
  ;;[1 1 1] Light Attack
  (`/Engine/EditorBlueprintResources/StandardMacros.DoOnce` false :!label _label
    (:`Completed`
      (`|PlayMontage` (`self.carachterMesh`) "/Game/Assets/Animations/HammerAttacks/AM_Horizontal_Attack.AM_Horizontal_Attack" 1.5
        (:`then`
          (set `self.attackIndex` 1)
          (`KismetArrayLibrary.Array_Clear` (`self.Hit`))
          (goto _label :!via `Reset`))))))

(event `Sphere Trace`
  (bind _returnvalue (`SceneComponent.K2_GetComponentLocation` (`/Game/Assets/BluePrints/MainCharacter/BP_MainCharacter.AoETrace` (`self.Character_REF`))))
  ;[0.1594 1 0.332] Sphere Trace (For Hammer Thrust)
  (`KismetArrayLibrary.Array_Clear` (`self.Hit`))
  (bind _outhits (`KismetSystemLibrary.SphereTraceMultiForObjects` _returnvalue _returnvalue 300.0 (`self.Object Types`) false (`|MakeArray` null :!type "Actor Object Reference")))
  (for _array_element _outhits
    (bind (_bblockinghit _binitialoverlap _time _distance _location _impactpoint _normal _impactnormal _physmat _hitactor) (`GameplayStatics.BreakHitResult` _array_element))
    (bind _asbpidamage_recievers (cast `/Game/Assets/BluePrints/Interfaces/BPIDamageRecievers` _hitactor))
    (if (not (`KismetArrayLibrary.Array_Contains` (`self.Hit`) _asbpidamage_recievers))
      (message `/Game/Assets/BluePrints/Interfaces/BPIDamageRecievers.Knockback` _hitactor (`Actor.K2_GetActorLocation` (`self.Character_REF`)) 75.0 500.0)
      (message `/Game/Assets/BluePrints/Interfaces/BPIDamageRecievers.TakeDamage` _hitactor 20.0)
      (`KismetArrayLibrary.Array_Add` (`self.Hit`) _asbpidamage_recievers))))

(event `Light Hammer Attack`
  ;[0.1594 1 0.332] Combo System
  ;;[1 1 1] Light Hammer Attack
  (set `self.Damage` 15.0)
  (set `self.Launch` 200.0)
  (set `self.Knockback` 1000.0)
  (if (`self.isAttacking?`)
    (set `self.saveAttack?` true)
    (else
      (set `self.isAttacking?` true)
      (`self.Attack 1`))))

(event `Light Attack Overhead`
  ;[0.1594 1 0.332] Combo System
  ;;[1 1 1] Light Attack Overhead
  (`/Engine/EditorBlueprintResources/StandardMacros.DoOnce` false :!label _label_2
    (:`Completed`
      (`|PlayMontage` (`self.carachterMesh`) "/Game/Assets/Animations/HammerAttacks/AM_Overhead_Attack.AM_Overhead_Attack" 1.3
        (:`then`
          (set `self.attackIndex` 2)
          (`KismetArrayLibrary.Array_Clear` (`self.Hit`))
          (goto _label_2 :!via `Reset`))))))

(event `FollowUpAttack`
  ;[0.1594 1 0.332] Combo System
  ;;[1 1 1] Follow up Attack
  (`self.Light Attack Overhead`))

(event `Charge Attack`
  ;[0.1594 1 0.332] Combo System
  ;;[1 1 1] Charge Attack
  (`/Engine/EditorBlueprintResources/StandardMacros.DoOnce` false :!label _label_3
    (:`Completed`
      (`KismetSystemLibrary.Delay` 0.1)
      (`|PlayMontage` (`self.carachterMesh`) "/Game/Assets/Animations/HammerAttacks/OLD/AM_Attack3.AM_Attack3"
        (:`then`
          (`KismetArrayLibrary.Array_Clear` (`self.Hit`))
          (goto _label_3 :!via `Reset`))))))

(event `FollowUpAttackWindow`
  ;[0.1594 1 0.332] Combo System
  ;;[1 1 1] Timing window
  (set `self.secondAttack?` true)
  (`KismetSystemLibrary.Delay` 0.28)
  (set `self.secondAttack?` false))

(event `Start Hammer Trace`
  ;[0.159 1 0.3325] Hammer Trace
  (bind _returnvalue (`KismetSystemLibrary.K2_SetTimerDelegate` (delegate `Hammer Trace Loop`) 0.001 true))
  (set `self.HammerTraceLoop` _returnvalue))

(event `Hammer Trace Loop`
  ;[0.159 1 0.3325] Hammer Trace
  (bind (_outhits _returnvalue) (`KismetSystemLibrary.SphereTraceMultiForObjects` (`SceneComponent.K2_GetComponentLocation` (`/Game/Assets/BluePrints/MainCharacter/BP_MainCharacter.HammerTopPoint` (`self.Character_REF`))) (`SceneComponent.K2_GetComponentLocation` (`/Game/Assets/BluePrints/MainCharacter/BP_MainCharacter.HammerBottomPoint` (`self.Character_REF`))) 25.0 (`self.Object Types`) false (`|MakeArray` null :!type "Actor Object Reference")))
  (for _array_element _outhits
    (if _returnvalue
      (bind (_bblockinghit _binitialoverlap _time _distance _location _impactpoint _normal _impactnormal _physmat _hitactor) (`GameplayStatics.BreakHitResult` _array_element))
      (if (`KismetSystemLibrary.DoesImplementInterface` _hitactor "/Game/Assets/BluePrints/Interfaces/BPIDamageRecievers.BPIDamageRecievers_C")
        ;;[1 1 1] Exchange for Cast to interface
        (bind _asbpidamage_recievers (cast `/Game/Assets/BluePrints/Interfaces/BPIDamageRecievers` _hitactor))
        (if (not (`KismetArrayLibrary.Array_Contains` (`self.Hit`) _asbpidamage_recievers))
          (`/Engine/EditorBlueprintResources/StandardMacros.DoOnce` false :!label _label_4
            (:`Completed`
              (bind _returnvalue_2 (`KismetSystemLibrary.Conv_InterfaceToObject` _asbpidamage_recievers))
              (message `/Game/Assets/BluePrints/Interfaces/BPIDamageRecievers.Knockback` _returnvalue_2 (`Actor.K2_GetActorLocation` (`self.Character_REF`)) (`self.Knockback`) (`self.Launch`))
              (message `/Game/Assets/BluePrints/Interfaces/BPIDamageRecievers.TakeDamage` _returnvalue_2 (`self.Damage`))
              (`KismetArrayLibrary.Array_Add` (`self.Hit`) _asbpidamage_recievers)
              (goto _label_4 :!via `Reset`))))))))

(event `Light Attack Combo`
  ;[0.1594 1 0.332] Combo System
  ;;[1 1 1] Combo Continue
  (if (`self.saveAttack?`)
    (set `self.saveAttack?` false)
    (else
      (`self.Stop Combo`))))

(event `Stop Combo`
  ;[0.1594 1 0.332] Combo System
  ;;[1 1 1] Stop Combo/Attack
  (set `self.isAttacking?` false)
  (set `self.attackIndex` 0))

(event `Stop Hammer Trace`
  ;[0.159 1 0.3325] Hammer Trace
  (`KismetSystemLibrary.K2_ClearAndInvalidateTimerHandle` (`self.HammerTraceLoop`)))

(event `Heavy Hammer Attack`
  ;[0.1594 1 0.332] Combo System
  ;;[1 1 1] Heavy Hammer Attack
  (if (`self.isSlamming?`)
    _
    (elif (`self.isAttacking?`)
      (set `self.saveAttack?` true)
      (else
        (set `self.isAttacking?` true)
        (set `self.Damage` 50.0)
        (set `self.Knockback` 1000.0)
        (set `self.Launch` 500.0)
        (`self.Charge Attack`)))))

(event `Play Rupture Effect`
  (bind _character_ref (`self.Character_REF`))
  (bind (_returnvalue_x _returnvalue_y _returnvalue_z) (`KismetMathLibrary.BreakVector` (`Actor.K2_GetActorLocation` _character_ref)))
  (bind (_returnvalue_x_2 _returnvalue_y_2) (`KismetMathLibrary.BreakVector` (* (`Actor.GetActorForwardVector` _character_ref) 100.0)))
  (bind (_returnvalue_x_3 _returnvalue_y_3) (`KismetMathLibrary.BreakVector` (+ (`SceneComponent.K2_GetComponentLocation` (`/Game/Assets/BluePrints/MainCharacter/BP_MainCharacter.HammerBottomPoint` _character_ref)) (`KismetMathLibrary.MakeVector` _returnvalue_x_2 _returnvalue_y_2))))
  ;[1 1 1] Rupture
  (bind _returnvalue (`GameplayStatics.GetActorOfClass` "/Game/Assets/BluePrints/BP_Spells/BaseClass/BP_Rupture_Child.BP_Rupture_Child_C"))
  (message `/Game/Assets/BluePrints/BP_Spells/BaseClass/BPI_SpellEffects.CastSpell` _returnvalue (0.0 0.0 0.0) (`Actor.K2_GetActorRotation` _character_ref) null (`KismetMathLibrary.MakeVector` _returnvalue_x_3 _returnvalue_y_3 (- _returnvalue_z 100.0)) 0.0))

(event `SlamAttack`
  (bind _character_ref (`self.Character_REF`))
  ;[1 1 1] Slam Attack
  (if (not (`self.isSlamming?`))
    (set `self.isSlamming?` true)
    (`Character.LaunchCharacter` _character_ref (0.0 0.0 2000.0) false true)
    (`Character.PlayAnimMontage` _character_ref "/Game/Assets/Animations/HammerAttacks/AM_Slam_Attack.AM_Slam_Attack" 1.7 "None")
    (`self.Stop Combo`)))