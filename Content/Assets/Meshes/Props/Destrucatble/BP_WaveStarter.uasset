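; Destructible crystal prop that starts enemy waves through the level's BP_WaveManager when its health runs out.
; Each hit shakes the camera, plays splatter and sound, and briefly swaps to flash materials using a retriggerable delay.
; Breaking fires larger effects once, moves the capsule to an offset hide position and calls StartWaves.
; Optional respawn restores health after a random delay, animates position with a timeline and re-arms the DoOnce.
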(event `self.ReceiveBeginPlay`
  (bind _returnvalue (`SceneComponent.K2_GetComponentLocation` (`self.Capsule`)))
  (set `self.MaxHP` (`self.Health`))
  (set `self.SpawnPosition` _returnvalue)
  (set `self.HidePosition` (+ _returnvalue (`self.MoveAmmount`)))
  (bind _returnvalue_2 (`GameplayStatics.GetActorOfClass` "/Game/AI/WaveLogic/BP_WaveManager.BP_WaveManager_C"))
  (set `self.WaveManager` _returnvalue_2))

(event `/Game/Assets/BluePrints/Interfaces/BPIDamageRecievers.TakeDamage`
  (params (`Damage Taken` :type "Float (double-precision)") (PoiseDamage :type "Float (double-precision)"))
  (bind _returnvalue (`SceneComponent.K2_GetComponentLocation` (`self.Capsule`)))
  (`PlayerCameraManager.StartCameraShake` :`self` (`PlayerController.PlayerCameraManager` (`GameplayStatics.GetPlayerController` 0)) :`ShakeClass` "/Game/Assets/VFX/CameraShake.CameraShake_C" :`Scale` 0.4)
  (bind _output_get (set `self.Health` (- (`self.Health`) `Damage Taken`)))
  (if (> _output_get 0.0)
    (bind _returnvalue_2 (`NiagaraFunctionLibrary.SpawnSystemAtLocation` "/Game/Assets/Meshes/Props/Destrucatble/NS_CrystalSplatter.NS_CrystalSplatter" (`SceneComponent.K2_GetComponentLocation` (`self.Capsule`))))
    (`PrimitiveComponent.SetRenderCustomDepth` _returnvalue_2 true)
    (`PrimitiveComponent.SetCustomDepthStencilValue` _returnvalue_2 (`PrimitiveComponent.CustomDepthStencilValue` (`self.Crystal2_LP`)))
    (`GameplayStatics.PlaySoundAtLocation` "/Game/SoundFX/MetaSounds/MS_CrystalSpawnerHit.MS_CrystalSpawnerHit" (`SceneComponent.K2_GetComponentLocation` (`self.Capsule`)) (struct) 1.2 1.0 0.2 null null null null)
    (`PrimitiveComponent.SetMaterial` (`self.Crystal_LP1`) 0 "/Game/Assets/Meshes/Props/Destrucatble/MI_Crystal_HitEffect1.MI_Crystal_HitEffect1")
    (`PrimitiveComponent.SetMaterial` (`self.Crystal_LP2`) 0 "/Game/Assets/Meshes/Props/Destrucatble/MI_Crystal_HitEffect1.MI_Crystal_HitEffect1")
    (`PrimitiveComponent.SetMaterial` (`self.Crystal_LP3`) 0 "/Game/Assets/Meshes/Props/Destrucatble/MI_Crystal_HitEffect1.MI_Crystal_HitEffect1")
    (`PrimitiveComponent.SetMaterial` (`self.Crystal2_LP`) 0 "/Game/Assets/Meshes/Props/Destrucatble/MI_Crystal_HitEffect2.MI_Crystal_HitEffect2")
    (`KismetSystemLibrary.RetriggerableDelay` 0.2)
    (`PrimitiveComponent.SetMaterial` (`self.Crystal_LP1`) 0 "/Game/Assets/Meshes/Props/Crystals/Crystal1/MI_Crystal1.MI_Crystal1")
    (`PrimitiveComponent.SetMaterial` (`self.Crystal_LP2`) 0 "/Game/Assets/Meshes/Props/Crystals/Crystal1/MI_Crystal1.MI_Crystal1")
    (`PrimitiveComponent.SetMaterial` (`self.Crystal_LP3`) 0 "/Game/Assets/Meshes/Props/Crystals/Crystal1/MI_Crystal1.MI_Crystal1")
    (`PrimitiveComponent.SetMaterial` (`self.Crystal2_LP`) 0 "/Game/Assets/Meshes/Props/Crystals/Crystal2/MI_Crystal2.MI_Crystal2")
    (else
      (`/Engine/EditorBlueprintResources/StandardMacros.DoOnce` false :!label _label
        (:`Completed`
          (`PlayerCameraManager.StartCameraShake` :`self` (`PlayerController.PlayerCameraManager` (`GameplayStatics.GetPlayerController` 0)) :`ShakeClass` "/Game/Assets/VFX/CameraWaveShake.CameraWaveShake_C" :`Scale` 0.5)
          (bind _returnvalue_3 (`NiagaraFunctionLibrary.SpawnSystemAtLocation` "/Game/Assets/Meshes/Props/Destrucatble/NS_CrystalSplatter_Large.NS_CrystalSplatter_Large" _returnvalue))
          (`PrimitiveComponent.SetRenderCustomDepth` _returnvalue_3 true)
          (`PrimitiveComponent.SetCustomDepthStencilValue` _returnvalue_3 (`PrimitiveComponent.CustomDepthStencilValue` (`self.Crystal2_LP`)))
          (bind _returnvalue_4 (`NiagaraFunctionLibrary.SpawnSystemAtLocation` "/Game/Assets/Meshes/Props/Destrucatble/NS_CrystalSplatter_Gigantic.NS_CrystalSplatter_Gigantic" _returnvalue))
          (`GameplayStatics.PlaySound2D` "/Game/SoundFX/MetaSounds/MS_CrystalSpawnerHit.MS_CrystalSpawnerHit" 1.2 1.0 0.2 null null)
          (`PrimitiveComponent.SetRenderCustomDepth` _returnvalue_4 true)
          (`PrimitiveComponent.SetCustomDepthStencilValue` _returnvalue_4 (`PrimitiveComponent.CustomDepthStencilValue` (`self.Crystal2_LP`)))
          (`GameplayStatics.PlaySound2D` "/Game/SoundFX/MetaSounds/Implemented/MS_CrystalBreak.MS_CrystalBreak" 2.0 1.0 0.0 null null)
          (`SceneComponent.K2_SetWorldLocation` (`self.Capsule`) (`self.HidePosition`) false false)
          (`/Game/AI/WaveLogic/BP_WaveManager.StartWaves` (`self.WaveManager`))
          (if (`self.Respawn?`)
            (`KismetSystemLibrary.Delay` (`KismetMathLibrary.RandomFloatInRange` (`self.RespawnMin`) (`self.RespawnMax`)))
            (set `self.Health` (`self.MaxHP`))
            (bind (_direction _alpha) (`Timeline|Respawn`)
              (:`Update`
                (`SceneComponent.K2_SetWorldLocation` (`self.Capsule`) (`KismetMathLibrary.VLerp` (`self.SpawnPosition`) (`self.HidePosition`) _alpha) false false))
              (:`Finished`
                (goto _label :!via `Reset`)))))))))

(fn `UserConstructionScript`)