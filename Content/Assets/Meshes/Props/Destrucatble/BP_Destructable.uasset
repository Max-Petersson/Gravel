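; Destructible crystal prop that loses health when damaged, with an optional timed respawn.
; Each hit shakes the camera, and non-lethal hits spawn a splatter effect and briefly flash the two crystal meshes with hit materials.
; At zero health a DoOnce spawns larger splatter and moves the capsule to an offset hiding spot rather than destroying it.
; If respawn is enabled, health refills after a delay and a timeline animates the position before re-arming.
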(event `self.ReceiveBeginPlay`
  (bind _returnvalue (`SceneComponent.K2_GetComponentLocation` (`self.Capsule`)))
  (set `self.MaxHP` (`self.Health`))
  (set `self.SpawnPosition` _returnvalue)
  (set `self.HidePosition` (+ _returnvalue (`self.MoveAmmount`))))

(event `/Game/Assets/BluePrints/Interfaces/BPIDamageRecievers.TakeDamage`
  (params (`Damage Taken` :type "Float (double-precision)"))
  (bind _returnvalue (`SceneComponent.K2_GetComponentLocation` (`self.Capsule`)))
  (`PlayerCameraManager.StartCameraShake` :`self` (`PlayerController.PlayerCameraManager` (`GameplayStatics.GetPlayerController` 0)) :`ShakeClass` "/Game/Assets/VFX/CameraShake.CameraShake_C" :`Scale` 0.2)
  (bind _output_get (set `self.Health` (- (`self.Health`) `Damage Taken`)))
  (if (> _output_get 0.0)
    (`NiagaraFunctionLibrary.SpawnSystemAtLocation` "/Game/Assets/Meshes/Props/Destrucatble/NS_CrystalSplatter.NS_CrystalSplatter" (`SceneComponent.K2_GetComponentLocation` (`self.Capsule`)))
    (`PrimitiveComponent.SetMaterial` (`self.Crystal_LP1`) 0 "/Game/Assets/Meshes/Props/Destrucatble/MI_Crystal_HitEffect1.MI_Crystal_HitEffect1")
    (`PrimitiveComponent.SetMaterial` (`self.Crystal2_LP`) 0 "/Game/Assets/Meshes/Props/Destrucatble/MI_Crystal_HitEffect2.MI_Crystal_HitEffect2")
    (`KismetSystemLibrary.RetriggerableDelay` 0.1)
    (`PrimitiveComponent.SetMaterial` (`self.Crystal_LP1`) 0 "/Game/Assets/Meshes/Props/Crystals/Crystal1/MI_Crystal1.MI_Crystal1")
    (`PrimitiveComponent.SetMaterial` (`self.Crystal2_LP`) 0 "/Game/Assets/Meshes/Props/Crystals/Crystal2/MI_Crystal2.MI_Crystal2")
    (else
      (`/Engine/EditorBlueprintResources/StandardMacros.DoOnce` false :!label _label
        (:`Completed`
          (`NiagaraFunctionLibrary.SpawnSystemAtLocation` "/Game/Assets/Meshes/Props/Destrucatble/NS_CrystalSplatter_Large.NS_CrystalSplatter_Large" _returnvalue)
          (`NiagaraFunctionLibrary.SpawnSystemAtLocation` "/Game/Assets/Meshes/Props/Destrucatble/NS_CrystalSplatter.NS_CrystalSplatter" _returnvalue)
          (`SceneComponent.K2_SetWorldLocation` (`self.Capsule`) (`self.HidePosition`) false false)
          (if (`self.Respawn?`)
            (`KismetSystemLibrary.Delay` (`self.Respawntimer`))
            (set `self.Health` (`self.MaxHP`))
            (bind (_direction _alpha) (`Timeline|Respawn`)
              (:`Update`
                (`SceneComponent.K2_SetWorldLocation` (`self.Capsule`) (`KismetMathLibrary.VLerp` (`self.SpawnPosition`) (`self.HidePosition`) _alpha) false false))
              (:`Finished`
                (goto _label :!via `Reset`)))))))))

(fn `UserConstructionScript`)