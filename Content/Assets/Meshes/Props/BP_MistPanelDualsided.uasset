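; Mist panel prop: a plane mesh showing two-sided animated fog, tunable per placed instance.
; The construction script creates a dynamic instance of M_FogPlane_TwoSided on the plane and pushes the actor's variables into it.
; These drive panning speed, color, distance and depth fading, softness and noise zoom.
; The event graph is empty, so all setup happens at construction with no runtime logic.
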(fn `UserConstructionScript`
  (bind _returnvalue (`PrimitiveComponent.CreateDynamicMaterialInstance` (`self.SimplePlane`) 0 "/Game/Assets/Materials/FogMaterials/M_FogPlane_TwoSided.M_FogPlane_TwoSided" "Initialized_FogMat"))
  (set `self.Fog Plane Mat` _returnvalue)
  (`|ExecutionSequence`
    (:`then_0`
      (`MaterialInstanceDynamic.SetScalarParameterValue` (`self.Fog Plane Mat`) "PanningSpeedMulti" (`self.Speed_Multiplyer`)))
    (:`then_1`
      (`MaterialInstanceDynamic.SetScalarParameterValue` (`self.Fog Plane Mat`) "SpeedX" (`self.Speed_X`)))
    (:`then_2`
      (`MaterialInstanceDynamic.SetScalarParameterValue` (`self.Fog Plane Mat`) "SpeedY" (`self.Speed_Y`)))
    (:`then_3`
      (`MaterialInstanceDynamic.SetVectorParameterValue` (`self.Fog Plane Mat`) "Color" (`self.Color`)))
    (:`then_4`
      (`MaterialInstanceDynamic.SetScalarParameterValue` (`self.Fog Plane Mat`) "FogStartFadeDistance" (`self.Fade_Start_Distance`)))
    (:`then_5`
      (`MaterialInstanceDynamic.SetScalarParameterValue` (`self.Fog Plane Mat`) "DepthFadeDistance" (`self.Fade_Depth_Distance`)))
    (:`then_6`
      (`MaterialInstanceDynamic.SetScalarParameterValue` (`self.Fog Plane Mat`) "SoftnessMulti" (`self.Softness_Multiplyer`)))
    (:`then_7`
      (`MaterialInstanceDynamic.SetScalarParameterValue` (`self.Fog Plane Mat`) "NoiseZoom" (`self.Zoom`)))))