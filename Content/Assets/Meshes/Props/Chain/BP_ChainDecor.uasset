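; BP_ChainDecor is a decorative physics chain prop whose length is set by ChainAmmount.
; The construction script derives link spacing and joint offset from the template components (links 1, 2 and PhysicsConstraint).
; It then spawns simulating chain meshes, each joined to the previous link by a physics constraint with limited swing and twist and collision disabled between the pair.
; The event graph is unused.
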(fn `UserConstructionScript`
  (bind _2 (`self.2`))
  (bind (_returnvalue_location _returnvalue_rotation _returnvalue_scale) (`KismetMathLibrary.BreakTransform` (`SceneComponent.GetRelativeTransform` (`self.1`))))
  (bind _relativelocation (`SceneComponent.RelativeLocation` _2))
  ;[0.05098 0.05098 0.05098] Set Defult Variables
  (set `self.LastChain` _2)
  (set `self.last position` _relativelocation)
  (set `self.SeperationDistance` (+ (`SceneComponent.RelativeLocation` (`self.1`)) _relativelocation))
  (set `self.JointDistance` (- (`SceneComponent.RelativeLocation` (`self.PhysicsConstraint`)) _relativelocation))
  (for _ (range 1 (+ (`self.Chain Ammount`) 1))
    ;[0.05098 0.05098 0.05098] Create And Set New Chain Peice
    (bind _returnvalue (`AddComponent|NODE_AddStaticMeshComponent-0` :`RelativeTransform` (`KismetMathLibrary.MakeTransform` (+ (`self.last position`) (`self.SeperationDistance`)) _returnvalue_rotation _returnvalue_scale)))
    (bind _output_get (set `self.NewChain` _returnvalue))
    (`StaticMeshComponent.SetStaticMesh` _output_get "/Game/Assets/Meshes/Props/Chain/Chain_single.Chain_single")
    (bind _relativelocation_2 (`SceneComponent.RelativeLocation` _output_get))
    (set `self.last position` _relativelocation_2)
    ;[0.05098 0.05098 0.05098] Create And Set Chain Constraint Component
    (bind _returnvalue_2 (`AddComponent|NODE_AddPhysicsConstraintComponent-0` :`RelativeTransform` (`KismetMathLibrary.MakeTransform` (+ _relativelocation_2 (`self.JointDistance`)) (struct :`Pitch` -90.0))))
    (`PhysicsConstraintComponent.SetAngularSwing1Limit` _returnvalue_2 "ACM_Limited" 45.0)
    (`PhysicsConstraintComponent.SetAngularSwing2Limit` _returnvalue_2 "ACM_Limited" 45.0)
    (`PhysicsConstraintComponent.SetAngularTwistLimit` _returnvalue_2 "ACM_Limited" 45.0)
    (`PhysicsConstraintComponent.SetDisableCollision` _returnvalue_2 true)
    (`PhysicsConstraintComponent.SetConstrainedComponents` _returnvalue_2 (`self.LastChain`) "None" (`self.NewChain`) "None")
    (bind _output_get_2 (set `self.LastChain` (`self.NewChain`)))
    (`PrimitiveComponent.SetSimulatePhysics` _output_get_2 true)))